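; BP_Chicken_New is a farm chicken that counts down to a collectable product once fed and can patrol around its barn.
; Tick syncs the feed state with a Timer widget and, when the countdown hits zero, swaps the logo and timer for the product widget.
; Hovering a fed chicken shows the timer instead of the logo.
; PatrollingSheep loops AI moves to random navigable points near the barn, pausing after each arrival.
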(event Custom|Patrolling%20Sheep
  ;[1 1 1] PatrollingCode
  (if (not (Variables|Default|GetMoving))
    (AI|AIMoveTo self (.RandomLocation (Class|NavigationSystemV1|GetRandomPointinNavigableRadius (Transformation|GetActorLocation (Variables|Default|GetBarnRef)) (Variables|Default|GetPatrolRadius) 0 0)) (Variables|Default|GetBarnRef) 5.0 false
      (:then
        (Variables|Default|SetMoving true))
      (:OnSuccess
        (Utilities|FlowControl|Delay (Math|Random|RandomFloatinRange 2.0 5.0))
        (Variables|Default|SetMoving false)
        (CallFunction|PatrollingSheep))
      (:OnFail
        (Variables|Default|SetMoving false)
        (CallFunction|PatrollingSheep)))))

(event EventBeginPlay
  (bind _astimer (Utilities|Casting|CastToTimer (UserInterface|GetUserWidgetObject (Variables|Default|GetTimer))))
  (Variables|Default|SetWidgetTimerRef _astimer)
  (bind _asmilk_produced (Utilities|Casting|CastToMilkProduced (UserInterface|GetUserWidgetObject (Variables|Default|GetProduct))))
  (Variables|Default|SetWidgetFoodCollectRef _asmilk_produced)
  (Variables|/Script/Engine.PlayerController|SetbEnableMouseOverEvents (Game|GetPlayerController 0) true))

(event EventTick
  (params (DeltaSeconds :type Float%20%28single-precision%29))
  (bind _widgettimerref (Variables|Default|GetWidgetTimerRef))
  (bind _seconds (Variables|/Game/Inventory/UI/TimerUI/Timer.Timer_C|GetSeconds _widgettimerref))
  (Variables|/Game/Inventory/UI/TimerUI/Timer.Timer_C|SetIsFeed _widgettimerref (Variables|Default|GetIsFeed))
  (if (Variables|Default|GetIsFeed)
    (if (== _seconds (Variables|Default|GetSeconds))
      (Rendering|SetVisibility (Variables|Default|GetLogo) true false))
    (if (== _seconds 0)
      (Variables|Default|SetIsReady true)
      (bind _output_get (Variables|/Game/Inventory/UI/TimerUI/Timer.Timer_C|SetIsReady (Variables|Default|GetWidgetTimerRef) (Variables|Default|GetIsReady)))
      (if _output_get
        (Rendering|SetVisibility (Variables|Default|GetTimer) false false)
        (Rendering|SetVisibility (Variables|Default|GetProduct) true false)))
    (else
      (Rendering|SetVisibility (Variables|Default|GetProduct) false false)
      (Variables|Default|SetIsReady false)
      (Variables|/Game/Inventory/UI/TimerUI/Timer.Timer_C|SetIsReady (Variables|Default|GetWidgetTimerRef) (Variables|Default|GetIsReady)))))

(event MouseInput|EventActorBeginCursorOver
  (if (Variables|Default|GetIsFeed)
    (Rendering|SetVisibility (Variables|Default|GetLogo) false false)
    (Rendering|SetVisibility (Variables|Default|GetTimer) true false)))

(event MouseInput|EventActorEndCursorOver
  (if (Variables|Default|GetIsFeed)
    (Rendering|SetVisibility (Variables|Default|GetLogo) true false)
    (Rendering|SetVisibility (Variables|Default|GetTimer) false false)))

(fn ConstructionScript)