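; BP_Cow1 is a cow AI that patrols around a barn.
; PatrollingCow, started on BeginPlay, requests AI MoveTo with a random navigable point around BarnRef and also BarnRef as TargetActor, which takes precedence when valid.
; A Moving flag guards requests; success waits a random delay before repeating, while failure retries immediately.
; The owner cast that assigns BarnRef is disconnected, so this graph never sets it.
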(event Custom|Patrolling%20Cow
  (if (not (Variables|Default|GetMoving))
    (AI|AIMoveTo self (.RandomLocation (Class|NavigationSystemV1|GetRandomPointinNavigableRadius (Transformation|GetActorLocation (Variables|Default|GetBarnRef)) (Variables|Default|GetPatrolRadius) 0 0)) (Variables|Default|GetBarnRef) 1e+02 true
      (:then
        (Variables|Default|SetMoving true))
      (:OnSuccess
        (Utilities|FlowControl|Delay (Math|Random|RandomFloatinRange 2.0 5.0))
        (Variables|Default|SetMoving false)
        (CallFunction|PatrollingCow))
      (:OnFail
        (Variables|Default|SetMoving false)
        (CallFunction|PatrollingCow)))))

(event EventBeginPlay
  (Utilities|FlowControl|Sequence
    (:then_0
      _)
    (:then_1
      _))
  (CallFunction|PatrollingCow))

(fn ConstructionScript)