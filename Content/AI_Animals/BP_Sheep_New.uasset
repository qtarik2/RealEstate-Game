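; Sheep farm animal that wanders around its barn and produces wool once fed and its timer runs out.
; BeginPlay caches the Timer and Wool widgets from its widget components.
; Tick copies IsFeed to the timer widget and swaps the timer for the wool widget when Seconds hits zero, resetting while unfed.
; PatrollingSheep loops AI moves to random navmesh points near BarnRef, pausing randomly after each arrival.
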(event Custom|Patrolling%20Sheep
  ;[1 1 1] PatrollingCode
  (if (not (Variables|Default|GetMoving))
    (AI|AIMoveTo self (.RandomLocation (Class|NavigationSystemV1|GetRandomPointinNavigableRadius (Transformation|GetActorLocation (Variables|Default|GetBarnRef)) (Variables|Default|GetPatrolRadius) 0 0)) (Variables|Default|GetBarnRef) 5.0 false
      (:then
        (Variables|Default|SetMoving true))
      (:OnSuccess
        (Utilities|FlowControl|Delay (Math|Random|RandomFloatinRange 2.0 5.0))
        (Variables|Default|SetMoving false)
        (CallFunction|PatrollingSheep))
      (:OnFail
        (Variables|Default|SetMoving false)
        (CallFunction|PatrollingSheep)))))

(event EventBeginPlay
  (bind _astimer (Utilities|Casting|CastToTimer (UserInterface|GetUserWidgetObject (Variables|Default|GetTimer))))
  (Variables|Default|SetWidgetTimerRef _astimer)
  (bind _aswool (Utilities|Casting|CastToWool (UserInterface|GetUserWidgetObject (Variables|Default|GetProduct))))
  (Variables|Default|SetWidgetFoodCollectRef _aswool))

(event EventTick
  (params (DeltaSeconds :type Float%20%28single-precision%29))
  (bind _widgettimerref (Variables|Default|GetWidgetTimerRef))
  (Variables|/Game/Inventory/UI/TimerUI/Timer.Timer_C|SetIsFeed _widgettimerref (Variables|Default|GetIsFeed))
  (if (Variables|Default|GetIsFeed)
    (if (== (Variables|/Game/Inventory/UI/TimerUI/Timer.Timer_C|GetSeconds _widgettimerref) 0)
      (Variables|Default|SetIsReady true)
      (bind _output_get (Variables|/Game/Inventory/UI/TimerUI/Timer.Timer_C|SetIsReady (Variables|Default|GetWidgetTimerRef) (Variables|Default|GetIsReady)))
      (if _output_get
        (Rendering|SetVisibility (Variables|Default|GetTimer) false false)
        (Rendering|SetVisibility (Variables|Default|GetProduct) true false)))
    (else
      (Rendering|SetVisibility (Variables|Default|GetProduct) false false)
      (Rendering|SetVisibility (Variables|Default|GetTimer) true false)
      (Variables|Default|SetIsReady false)
      (Variables|/Game/Inventory/UI/TimerUI/Timer.Timer_C|SetIsReady (Variables|Default|GetWidgetTimerRef) false))))

(event MouseInput|EventActorBeginCursorOver)

(event MouseInput|EventActorEndCursorOver)

(fn ConstructionScript)