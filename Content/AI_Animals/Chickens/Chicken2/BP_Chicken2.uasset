(event OnTargetPerceptionUpdated(AIPerception)
  (params (Actor :type Actor%20Object%20Reference) (Stimulus :type AI%20Stimulus%20Structure))
  (if (not (Variables|Default|GetMoving))
    (AI|AIMoveTo self (.RandomLocation (Class|NavigationSystemV1|GetRandomPointinNavigableRadius (Transformation|GetActorLocation (Variables|Default|GetChickenRef)) (Variables|Default|GetPatrolRadius) 0 0)) (Variables|Default|GetChickenRef) 5.0 true
      (:then
        (Variables|Default|SetMoving true))
      (:OnSuccess
        (Utilities|FlowControl|Delay (Math|Random|RandomFloatinRange 2.0 5.0))
        (Variables|Default|SetMoving false)
        (CallFunction|PatrollingChicken))
      (:OnFail
        (Variables|Default|SetMoving false)
        (CallFunction|PatrollingChicken)))))

(event Custom|Patrolling%20Chicken
  (if (not (Variables|Default|GetMoving))
    (AI|AIMoveTo self (.RandomLocation (Class|NavigationSystemV1|GetRandomPointinNavigableRadius (Transformation|GetActorLocation (Variables|Default|GetChickenRef)) (Variables|Default|GetPatrolRadius) 0 0)) (Variables|Default|GetChickenRef) 5.0 true
      (:then
        (Variables|Default|SetMoving true))
      (:OnSuccess
        (Utilities|FlowControl|Delay (Math|Random|RandomFloatinRange 2.0 5.0))
        (Variables|Default|SetMoving false)
        (CallFunction|PatrollingChicken))
      (:OnFail
        (Variables|Default|SetMoving false)
        (CallFunction|PatrollingChicken)))))

(event EventBeginPlay
  (Utilities|FlowControl|Sequence
    (:then_0
      _)
    (:then_1
      _))
  (CallFunction|PatrollingChicken))

(fn ConstructionScript)