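; BP_Chicken is a farm chicken that wanders and runs a countdown once it has feed.
; A self-restarting AI MoveTo patrols around ChickenRef, pausing randomly after successful moves.
; Tick uses a Delay to count Seconds down; at zero it swaps widgets and icons, removes the timer UI, plays a sound, sets ChickenID and stops ticking.
; Cursor hover toggles two widgets during the countdown, and several disconnected leftover chains never run.
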(event Custom|Patrolling%20Chicken
  (if (not (Variables|Default|GetMoving))
    (AI|AIMoveTo self (.RandomLocation (Class|NavigationSystemV1|GetRandomPointinNavigableRadius (Transformation|GetActorLocation (Variables|Default|GetChickenRef)) (Variables|Default|GetPatrolRadius) 0 0)) (Variables|Default|GetChickenRef) 5.0 true
      (:then
        (Variables|Default|SetMoving true))
      (:OnSuccess
        (Utilities|FlowControl|Delay (Math|Random|RandomFloatinRange 2.0 5.0))
        (Variables|Default|SetMoving false)
        (CallFunction|PatrollingChicken))
      (:OnFail
        (Variables|Default|SetMoving false)
        (CallFunction|PatrollingChicken)))))

(event EventBeginPlay
  (Variables|/Script/Engine.PlayerController|SetbEnableMouseOverEvents (Game|GetPlayerController 0) true)
  (Rendering|SetVisibility (Variables|Default|GetWidget) false false)
  (Rendering|SetVisibility (Variables|Default|GetWidget1) false false)
  (Utilities|FlowControl|Sequence
    (:then_0
      _)
    (:then_1
      _))
  (CallFunction|PatrollingChicken))

(event EventTick
  (params (DeltaSeconds :type Float%20%28single-precision%29))
  (bind _widget (Variables|Default|GetWidget))
  (bind _foundwidgets (Widget|GetAllWidgetsOfClass "/Game/Inventory/UI/Animal_Building_Crop_UI/CropingUI_UnUsed.CropingUI_UnUsed_C" true))
  (if (Variables|Default|GetHas%20feed?)
    (Utilities|FlowControl|Delay 1.0)
    (if (> (Variables|Default|GetSeconds) 0)
      (bind _result (Math|Integer|DecrementInt (Variables|Default|GetSeconds))
        (:%20%20
          (Variables|Default|SetSeconds _result)
          (Utilities|FlowControl|Delay 0.0)
          (Rendering|SetVisibility (Variables|Default|GetWidget1) false false)
          (if (<= (Variables|Default|GetSeconds) 1)
            (Rendering|SetVisibility (Variables|Default|GetWidget1) false false)
            (if (< (Variables|Default|GetSeconds) 1)
              (if (>= (Variables|Default|GetSeconds) 0)
                (Rendering|SetVisibility _widget true false)
                (else
                  (Rendering|SetVisibility _widget false false)))
              (if (== (Variables|Default|GetSeconds) 0)
                (Rendering|SetVisibility (Variables|Default|GetWidget) false false)
                (if (== (Variables|Default|GetSeconds) 0)
                  (Rendering|SetVisibility (Variables|Default|GetWidget2) true false)
                  (Utilities|FlowControl|Delay 0.0)
                  (bind _foundwidgets_2 (Widget|GetAllWidgetsOfClass "/Game/Inventory/UI/TimerUI/TimerUI.TimerUI_C" true))
                  (Variables|Default|SetTimerUIRef (Utilities|Array|Get(acopy) _foundwidgets_2))
                  (bind _foundwidgets_3 (Widget|GetAllWidgetsOfClass "/Game/Inventory/UI/Animal_Building_Crop_UI/CropingUI_UnUsed.CropingUI_UnUsed_C" true))
                  (Variables|Default|SetCropUIRef (Utilities|Array|Get(acopy) _foundwidgets_3))
                  (if (== (Variables|Default|GetSeconds) 0)
                    (Widget|RemovefromParent (Variables|Default|GetTimerUIRef))
                    (Rendering|SetVisibility (Variables|Default|GetWidget1) false false)
                    (if (== (Variables|Default|GetSeconds) 0)
                      (Widget|SetVisibility (Variables|/Game/Inventory/UI/TimerUI/LoadingIcon.LoadingIcon_C|GetImage_202 (Variables|Default|GetLoadingIconRef)) "Hidden")
                      (if (== (Variables|Default|GetSeconds) 0)
                        (Widget|SetVisibility (Variables|/Game/Inventory/UI/TimerUI/HarvestingIcon/ChickenIcon.ChickenIcon_C|GetImage_202 (Variables|Default|GetCowIconRef)) "Visible")
                        (Audio|PlaySound2D "/Game/Sound_Effects/Chicken/Chicken5.Chicken5" 1.0 1.0 0.0 0 0)
                        (Variables|Default|SetChickenID 2)
                        (if (== (Variables|Default|GetSeconds) 0)
                          (Actor|Tick|SetActorTickEnabled false))))))))))))))

(event MouseInput|EventActorBeginCursorOver
  (if (> (Variables|Default|GetSeconds) 0)
    (Rendering|SetVisibility (Variables|Default|GetWidget) false false)
    (Rendering|SetVisibility (Variables|Default|GetWidget1) true false)
    (else
      (Rendering|SetVisibility (Variables|Default|GetWidget) false false)
      (Rendering|SetVisibility (Variables|Default|GetWidget1) false false))))

(event MouseInput|EventActorEndCursorOver
  (if (> (Variables|Default|GetSeconds) 0)
    (Rendering|SetVisibility (Variables|Default|GetWidget) true false)
    (Rendering|SetVisibility (Variables|Default|GetWidget1) false false)
    (else
      (Rendering|SetVisibility (Variables|Default|GetWidget) false false)
      (Rendering|SetVisibility (Variables|Default|GetWidget1) false false))))

(fn ConstructionScript)