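; BP_FishingSpot is a placeable fishing spot with a fish type, shown on its sign, and a catch chance.
; Its trigger enables input, the interact widget and a gate for the E key, which toggles fishing unless a catch is underway.
; Starting passes spot settings to the player's CFishing component, snaps the player to an arrow and chains cast, catch and recast montages on blend-out while fishing continues.
; An Empty spot only prints a message.
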(event OnComponentBeginOverlap(FishingTrigger)
  (params (OverlappedComponent :type Primitive%20Component%20Object%20Reference) (OtherActor :type Actor%20Object%20Reference) (OtherComp :type Primitive%20Component%20Object%20Reference) (OtherBodyIndex :type Integer) (bFromSweep :type Boolean) (SweepResult :type Hit%20Result%20Structure%20%28by%20ref%29))
  (bind _player (Variables|Default|GetPlayer))
  (bind _player_2 (Variables|Default|GetPlayer))
  (bind _fishtypes (Variables|Default|GetFishTypes))
  (bind _player_3 (Variables|Default|GetPlayer))
  (bind _c_fishing (Variables|/Game/RPGFishing/Blueprints/Player/BP_FishingPlayer.BP_FishingPlayer_C|GetC_Fishing _player))
  ;[1 1 1] Enable input and interaction if player overlaps box collision
  (if (== OtherActor (Variables|Default|GetPlayer))
    (Input|EnableInput (Game|GetPlayerController 0))
    (Rendering|SetVisibility (Variables|Default|GetInteractWidget) true false)
    ;[1 1 1] Set Catch Percent Chance and fish type, position player, update fishing state, cast line
    (Utilities|FlowControl|Gate true) ; enters at Open
  ))

(event OnComponentEndOverlap(FishingTrigger)
  (params (OverlappedComponent :type Primitive%20Component%20Object%20Reference) (OtherActor :type Actor%20Object%20Reference) (OtherComp :type Primitive%20Component%20Object%20Reference) (OtherBodyIndex :type Integer))
  (bind _player (Variables|Default|GetPlayer))
  (bind _player_2 (Variables|Default|GetPlayer))
  (bind _fishtypes (Variables|Default|GetFishTypes))
  (bind _player_3 (Variables|Default|GetPlayer))
  (bind _c_fishing (Variables|/Game/RPGFishing/Blueprints/Player/BP_FishingPlayer.BP_FishingPlayer_C|GetC_Fishing _player))
  ;[1 1 1] Enable input and interaction if player overlaps box collision
  (if (== OtherActor (Variables|Default|GetPlayer))
    (Input|DisableInput (Game|GetPlayerController 0))
    (Rendering|SetVisibility (Variables|Default|GetInteractWidget) false false)
    ;[1 1 1] Set Catch Percent Chance and fish type, position player, update fishing state, cast line
    (Utilities|FlowControl|Gate true) ; enters at Close
  ))

(event Custom|StartCatchFish
  (bind _player (Variables|Default|GetPlayer))
  (bind _c_fishing (Variables|/Game/RPGFishing/Blueprints/Player/BP_FishingPlayer.BP_FishingPlayer_C|GetC_Fishing _player))
  ;[1 1 1] Catch fish
  (if (Variables|/Game/RPGFishing/Blueprints/Components/C_Fishing.C_Fishing_C|GetIsFishing? _c_fishing)
    (if (not (Variables|/Game/RPGFishing/Blueprints/Components/C_Fishing.C_Fishing_C|GetCatchingFish? _c_fishing))
      (Variables|/Game/RPGFishing/Blueprints/Components/C_Fishing.C_Fishing_C|SetCatchingFish? (Variables|/Game/RPGFishing/Blueprints/Player/BP_FishingPlayer.BP_FishingPlayer_C|GetC_Fishing (Variables|Default|GetPlayer)) true)
      (Animation|Montage|PlayMontage (Variables|/Script/Engine.Character|GetMesh (Variables|Default|GetPlayer)) "/Game/RPGFishing/Animations/Montages/AM_CatchFish.AM_CatchFish"
        (:OnBlendOut
          (CallFunction|ReTRiggerCast))))))

(event Custom|ReTriggerCast
  (bind _player (Variables|Default|GetPlayer))
  ;[1 1 1] Re-cast line
  (Variables|/Game/RPGFishing/Blueprints/Components/C_Fishing.C_Fishing_C|SetCatchingFish? (Variables|/Game/RPGFishing/Blueprints/Player/BP_FishingPlayer.BP_FishingPlayer_C|GetC_Fishing _player) false)
  (Animation|Montage|PlayMontage (Variables|/Script/Engine.Character|GetMesh _player) "/Game/RPGFishing/Animations/Montages/AM_Recast.AM_Recast"
    (:OnBlendOut
      ;[1 1 1] Start Catching Fish If Still Fishing
      (if (Variables|/Game/RPGFishing/Blueprints/Components/C_Fishing.C_Fishing_C|GetIsFishing? (Variables|/Game/RPGFishing/Blueprints/Player/BP_FishingPlayer.BP_FishingPlayer_C|GetC_Fishing (Variables|Default|GetPlayer)))
        (CallFunction|StartCatchFish)))))

(event EventBeginPlay
  ;[1 1 1] Begin Play
  (Rendering|Components|TextRender|SetText (Variables|Default|GetSignText) (Utilities|Text|ToText(String) (Utilities|String|EnumtoString (Variables|Default|GetFishTypes))))
  ;;[1 1 1] Change Cast And Variable Type To Your Player Character
  (bind _asbp_fishing_player (Utilities|Casting|CastToBP_FishingPlayer (Game|GetPlayerCharacter 0)))
  (Variables|Default|SetPlayer _asbp_fishing_player))

(event Input|KeyboardEvents|E
  (params (Key :type Key%20Structure))
  (bind _player (Variables|Default|GetPlayer))
  (bind _player_2 (Variables|Default|GetPlayer))
  (bind _fishtypes (Variables|Default|GetFishTypes))
  (bind _player_3 (Variables|Default|GetPlayer))
  (bind _c_fishing (Variables|/Game/RPGFishing/Blueprints/Player/BP_FishingPlayer.BP_FishingPlayer_C|GetC_Fishing _player))
  ;[1 1 1] Interact Key
  (:Pressed
    ;[1 1 1] Set Catch Percent Chance and fish type, position player, update fishing state, cast line
    (Utilities|FlowControl|Gate true
      (:Exit
        (Variables|/Game/RPGFishing/Blueprints/Components/C_Fishing.C_Fishing_C|SetCatchPercentChance _c_fishing (Variables|Default|GetCatchPercentChance))
        (Variables|/Game/RPGFishing/Blueprints/Components/C_Fishing.C_Fishing_C|SetCurrentFishingType _c_fishing _fishtypes)
        (switch Utilities|FlowControl|Switch|SwitchonE_FishTypes _fishtypes
          (:NewEnumerator0
            (Development|PrintString "There Are Currently No More Fish Here."))
          (:NewEnumerator1
            (if (not (Variables|/Game/RPGFishing/Blueprints/Components/C_Fishing.C_Fishing_C|GetIsFishing? _c_fishing)) :!label _label
              (Rendering|SetVisibility (Variables|Default|GetInteractWidget) false false)
              (Transformation|SetActorTransform (Variables|Default|GetPlayer) (Transformation|GetWorldTransform (Variables|Default|GetArrow)))
              (Default|UpdateFishingState (Variables|/Game/RPGFishing/Blueprints/Player/BP_FishingPlayer.BP_FishingPlayer_C|GetC_Fishing _player_2) true)
              (Animation|Montage|PlayMontage (Variables|/Script/Engine.Character|GetMesh _player_2) "/Game/RPGFishing/Animations/Montages/AM_PickupAndCast.AM_PickupAndCast"
                (:OnBlendOut
                  ;[1 1 1] Start Catching Fish If Still Fishing
                  (if (Variables|/Game/RPGFishing/Blueprints/Components/C_Fishing.C_Fishing_C|GetIsFishing? (Variables|/Game/RPGFishing/Blueprints/Player/BP_FishingPlayer.BP_FishingPlayer_C|GetC_Fishing (Variables|Default|GetPlayer)))
                    (CallFunction|StartCatchFish))))
              (else
                ;[1 1 1] Stop Fishing If Not In Middle Of Catching Fish
                (if (not (Variables|/Game/RPGFishing/Blueprints/Components/C_Fishing.C_Fishing_C|GetCatchingFish? _c_fishing))
                  (Animation|StopAnimMontage _player_3 0)
                  (Default|UpdateFishingState (Variables|/Game/RPGFishing/Blueprints/Player/BP_FishingPlayer.BP_FishingPlayer_C|GetC_Fishing _player_3) false)))))
          (:NewEnumerator2
            (goto _label))
          (:NewEnumerator3
            (goto _label))
          (:NewEnumerator4
            (goto _label)))))))

(fn ConstructionScript)