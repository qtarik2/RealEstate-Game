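; Anim notify that spawns the fishing pole in the player's hand at a set point in a fishing animation.
; When the mesh owner is a BP_FishingPlayer, it spawns a BP_FishingPole at the fishing_pole socket and snap-attaches it there.
; It stores the new pole on the C_Fishing component of player character 0, not of the animated owner.
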(fn GetNotifyName
  (return "ShowFishingPole"))

(fn ReceivedNotify
  (params (MeshComp :type Skeletal%20Mesh%20Component%20Object%20Reference) (Animation :type Anim%20Sequence%20Base%20Object%20Reference))
  ;[1 1 1] Spawn and attach fishing pole
  (bind _asbp_fishing_player (Utilities|Casting|CastToBP_FishingPlayer (Components|GetOwner MeshComp)))
  (bind _returnvalue (Game|SpawnActorfromClass "/Game/RPGFishing/Blueprints/BP_FishingPole.BP_FishingPole_C" (Transformation|GetSocketTransform (Variables|/Script/Engine.Character|GetMesh _asbp_fishing_player) "fishing_pole" "RTS_World") "Undefined" 0 0))
  (Variables|/Game/RPGFishing/Blueprints/Components/C_Fishing.C_Fishing_C|SetFishingPole (Actor|GetComponentbyClass (Game|GetPlayerCharacter 0) "/Game/RPGFishing/Blueprints/Components/C_Fishing.C_Fishing_C") _returnvalue)
  (Transformation|AttachComponentToComponent _returnvalue (Variables|/Script/Engine.Character|GetMesh _asbp_fishing_player) "fishing_pole" "SnapToTarget" "SnapToTarget" "KeepRelative" true)
  (return false))