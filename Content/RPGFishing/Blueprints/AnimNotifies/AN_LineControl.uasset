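; An anim notify that drives fishing line casting and reeling from the fishing player's animations.
; It finds the owning BP_FishingPlayer and calls its CFishing component.
; A Cast flag selects between casting the line and retracting it, with retraction followed by catching a fish of the current fishing type.
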(fn GetNotifyName
  (return "Cast/Reel Line"))

(fn ReceivedNotify
  (params (MeshComp :type Skeletal%20Mesh%20Component%20Object%20Reference) (Animation :type Anim%20Sequence%20Base%20Object%20Reference))
  ;[1 1 1] Cast or retract fishing line, catch fish after retracting
  (bind _asbp_fishing_player (Utilities|Casting|CastToBP_FishingPlayer (Components|GetOwner MeshComp)))
  (if (Variables|Default|GetCast?)
    (Default|CastLine (Variables|/Game/RPGFishing/Blueprints/Player/BP_FishingPlayer.BP_FishingPlayer_C|GetC_Fishing _asbp_fishing_player))
    (return false)
    (else
      (Default|RetractLine (Variables|/Game/RPGFishing/Blueprints/Player/BP_FishingPlayer.BP_FishingPlayer_C|GetC_Fishing _asbp_fishing_player))
      (Default|CatchFish (Variables|/Game/RPGFishing/Blueprints/Player/BP_FishingPlayer.BP_FishingPlayer_C|GetC_Fishing _asbp_fishing_player) (Variables|/Game/RPGFishing/Blueprints/Components/C_Fishing.C_Fishing_C|GetCurrentFishingType (Variables|/Game/RPGFishing/Blueprints/Player/BP_FishingPlayer.BP_FishingPlayer_C|GetC_Fishing _asbp_fishing_player))))))