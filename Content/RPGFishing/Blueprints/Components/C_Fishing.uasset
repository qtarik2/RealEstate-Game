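; Player fishing component that handles the fishing state, line casting and catch results.
; Entering fishing disables player movement and jumping; leaving restores them and destroys the pole, which also receives the cast and retract calls.
; A catch rolls against a percent chance, showing a result widget either way; success waits briefly, then increments that fish type in a placeholder struct inventory meant to be replaced.
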(event Custom|UpdateFishingState
  (params (IsFishing? :type Boolean))
  (bind _returnvalue (Game|GetPlayerCharacter 0))
  (bind _charactermovement (Variables|/Script/Engine.Character|GetCharacterMovement _returnvalue))
  ;[1 1 1] Disable movement and jumping while in fishing state
  (bind _output_get (Variables|Default|SetIsFishing? IsFishing?))
  (if _output_get
    (Pawn|Components|CharacterMovement|SetMovementMode _charactermovement "MOVE_None" 0)
    (Variables|/Script/Engine.CharacterMovementComponent|SetJumpZVelocity _charactermovement 0.0)
    (else
      (Pawn|Components|CharacterMovement|SetMovementMode _charactermovement "MOVE_Walking" 0)
      (Variables|/Script/Engine.CharacterMovementComponent|SetJumpZVelocity _charactermovement 4.2e+02)
      (bind _fishingpole (Variables|Default|GetFishingPole)
        (:then
          (Actor|DestroyActor _fishingpole))
        (:else)))))

(event Custom|CastLine
  ;[1 1 1] Cast/Retract Line
  (Default|CastLine (Variables|Default|GetFishingPole)))

(event Custom|RetractLine
  ;[1 1 1] Cast/Retract Line
  (Default|RetractLine (Variables|Default|GetFishingPole)))

(event Custom|CatchFish
  (params (FishType :type E_FishTypes%20Enum :default "NewEnumerator0"))
  (bind _fishinventory (Variables|Default|GetFishInventory))
  (bind (_trout _rainbowtrout _bass _shark) (Utilities|Struct|BreakS_FishInventory _fishinventory))
  ;[1 1 1] Add Fish To Inventory (would want to replace with your inventory add item event)
  (Utilities|CheckifFishWasCaught (Variables|Default|GetCatchPercentChance)
    (:Success
      (Utilities|FlowControl|Delay 2.0)
      (CallFunction|ShowFishCaughtText false)
      (switch Utilities|FlowControl|Switch|SwitchonE_FishTypes FishType
        (:NewEnumerator1
          (|AddFishToInventory _fishinventory _trout _rainbowtrout _bass _shark :!label _label))
        (:NewEnumerator2
          (goto _label AddRainbowTrout))
        (:NewEnumerator3
          (goto _label AddBass))
        (:NewEnumerator4
          (goto _label AddShark))))
    (:Fail
      (CallFunction|ShowFishCaughtText true))))

(fn ShowFishCaughtText
  (params (CatchFailed? :type Boolean))
  (bind _returnvalue (UserInterface|CreateWidget "/Game/RPGFishing/UI/WB_FishCaughtText.WB_FishCaughtText_C" 0 (Variables|Default|GetCurrentFishingType) CatchFailed?))
  (UserInterface|Viewport|AddtoViewport _returnvalue 0)
  (return))