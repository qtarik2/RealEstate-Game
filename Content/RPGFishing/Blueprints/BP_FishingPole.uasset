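; Fishing pole Blueprint that casts and retracts its line through a physics constraint.
; The CastLine and RetractLine events play the ExtendLine timeline forward from the start or backward from the end.
; The timeline update lerps the constraint's X, Y and Z linear limits between zero and LineLength, so line length is simulated as the allowed slack of the physics joint.
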(event Custom|RetractLine
  ;[1 1 1] Cast/Retract Line
  (Components|Timeline|ReversefromEnd (Variables|Default|GetExtendLine)))

(event Custom|CastLine
  ;[1 1 1] Cast/Retract Line
  (Components|Timeline|PlayfromStart (Variables|Default|GetExtendLine)))

(fn ConstructionScript)