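; BP_CarrotLoose is a ready-to-harvest carrot crop actor that the player collects by clicking it.
; BeginPlay enables click events on the player controller.
; A click adds carrots to ThirdPersonCharacter, destroys the actor, shows a pop-up widget, plays a harvest sound and awards XP through the character's LevelingSystem.
; An unconnected branch that resets and prints the game instance's PHPX value never runs.
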(event EventBeginPlay
  (Variables|/Script/Engine.PlayerController|SetbEnableClickEvents (Game|GetPlayerController 0) true))

(event MouseInput|EventActorOnClicked
  (params (ButtonPressed :type Key%20Structure :default "None"))
  (bind _asthird_person_character (Utilities|Casting|CastToThirdPersonCharacter (Game|GetPlayerCharacter 0)))
  (Variables|/Game/ThirdPersonBP/Blueprints/ThirdPersonCharacter.ThirdPersonCharacter_C|SetAmountOfCarrot _asthird_person_character (+ (Variables|/Game/ThirdPersonBP/Blueprints/ThirdPersonCharacter.ThirdPersonCharacter_C|GetAmountOfCarrot _asthird_person_character) 100))
  (Actor|DestroyActor)
  (bind _returnvalue (UserInterface|CreateWidget "/Game/Inventory/UI/PopUp_Menu/CropsPopUPs/CarrotPlantPopUpMsg.CarrotPlantPopUpMsg_C"))
  (UserInterface|Viewport|AddtoPlayerScreen _returnvalue)
  (Audio|PlaySound2D "/Game/Sound_Effects/CropingAndHarvestingCropsSounds/HarvestingSound/Harvest_Crop_Activities_2.Harvest_Crop_Activities_2" 1.0 1.0 0.0 0 0)
  (Default|AddXP (Variables|/Game/ThirdPersonBP/Blueprints/ThirdPersonCharacter.ThirdPersonCharacter_C|GetLevelingSystem _asthird_person_character) 2e+02))

(fn ConstructionScript)