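; Clickable loose asparagus crop actor that the player harvests into their asparagus count.
; On click, it adds a fixed amount to the ThirdPersonCharacter's asparagus total and destroys itself, then shows a pop-up widget, plays a harvest sound and awards XP through the character's LevelingSystem.
; The box overlap event is empty, and a GameInstance PHPX reset is left disconnected.
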(event OnComponentBeginOverlap(box)
  (params (OverlappedComponent :type Primitive%20Component%20Object%20Reference) (OtherActor :type Actor%20Object%20Reference) (OtherComp :type Primitive%20Component%20Object%20Reference) (OtherBodyIndex :type Integer) (bFromSweep :type Boolean) (SweepResult :type Hit%20Result%20Structure%20%28by%20ref%29)))

(event EventBeginPlay)

(event Collision|EventActorBeginOverlap
  (params (OtherActor :type Actor%20Object%20Reference)))

(event EventTick
  (params (DeltaSeconds :type Float%20%28single-precision%29)))

(event MouseInput|EventActorOnClicked
  (params (ButtonPressed :type Key%20Structure :default "None"))
  (bind _asthird_person_character (Utilities|Casting|CastToThirdPersonCharacter (Game|GetPlayerCharacter 0)))
  (Variables|/Game/ThirdPersonBP/Blueprints/ThirdPersonCharacter.ThirdPersonCharacter_C|SetAmountofAsparagus _asthird_person_character (+ (Variables|/Game/ThirdPersonBP/Blueprints/ThirdPersonCharacter.ThirdPersonCharacter_C|GetAmountofAsparagus _asthird_person_character) 315))
  (Actor|DestroyActor)
  (bind _returnvalue (UserInterface|CreateWidget "/Game/Inventory/UI/PopUp_Menu/CropsPopUPs/AsparagusPlantPopUp.AsparagusPlantPopUp_C" (Game|GetPlayerController 0)))
  (UserInterface|Viewport|AddtoPlayerScreen _returnvalue)
  (Audio|PlaySound2D "/Game/Sound_Effects/CropingAndHarvestingCropsSounds/HarvestingSound/Harvest_Crop_Activities_2.Harvest_Crop_Activities_2" 1.0 1.0 0.0 0 0)
  (Default|AddXP (Variables|/Game/ThirdPersonBP/Blueprints/ThirdPersonCharacter.ThirdPersonCharacter_C|GetLevelingSystem _asthird_person_character) 3e+01))

(fn ConstructionScript)