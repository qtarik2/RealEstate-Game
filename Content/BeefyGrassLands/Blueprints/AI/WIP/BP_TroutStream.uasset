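; Work-in-progress trout school that scatters instanced static meshes through a box volume at construction and makes them flee from reported locations.
; SetTraceLocation queues points; GetInstanceCollisions flags instances within an awareness sphere, and UpdateTroutInstances moves them using per-instance velocity and decaying acceleration.
; The timers driving both updates are disconnected from BeginPlay.
; Turn steering and scale-packed motion data are unfinished, and stored target locations are never read.
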(event EventBeginPlay)

(event Collision|EventActorBeginOverlap
  (params (OtherActor :type Actor%20Object%20Reference)))

(fn ConstructionScript
  (CallFunction|MakeInstances))

(fn UpdateTroutLocation
  (bind _returnvalue (Utilities|Time|GetGameTimeinSeconds))
  (CallFunction|UpdateTroutInstances (- (Utilities|Time|GetGameTimeinSeconds) (Variables|Default|GetTime)))
  (Variables|Default|SetTime _returnvalue)
  (Utilities|Array|SetArrayElem (Variables|Default|GetTimeOfLastUpdate) (Variables|Default|GetInstanceUpdateCount) _returnvalue)
  (bind _result (Math|Integer|IncrementInt (Variables|Default|GetInstanceUpdateCount))
    (:%20%20
      (Variables|Default|SetInstanceUpdateCount (Math|Integer|%(Integer) _result (Variables|Default|GetInstance%20Count))))))

(fn MakeInstances
  (bind _spawn_area (Variables|Components|GetSpawn%20Area))
  (bind _returnvalue (Transformation|GetWorldTransform _spawn_area))
  (Components|Box|SetBoxExtent (Variables|Components|GetSpawn%20Area) (Math|Vector|MakeVector (Variables|Default|GetVolumeX) (Variables|Default|GetVolumeY) (Variables|Default|GetVolumeZ)) true)
  (Components|InstancedStaticMesh|ClearInstances (Variables|Components|GetInstancedStaticMesh))
  (for _index (range 0 (- (Variables|Default|GetInstance%20Count) 1))
    (LocalVariables|SetNewLocation (Math|Transform|TransformLocation _returnvalue (Math|Vector|RotateVector (Math|Transform|TransformLocation (Math|Transform|InvertTransform _returnvalue) (Math|Random|RandomPointinBoundingBox (Transformation|GetWorldLocation _spawn_area) (Variables|/Script/Engine.BoxComponent|GetBoxExtent _spawn_area))) (Math|Transform|TransformRotation _returnvalue "0, 0, 0"))))
    (Class|InstancedStaticMeshComponent|AddInstanceWorldSpace (Variables|Components|GetInstancedStaticMesh) (Math|Transform|MakeTransform (LocalVariables|GetNewLocation) (Math|Rotator|MakeRotator 0.0 0.0 (+ (.yaw (Transformation|GetWorldRotation (Variables|Components|GetSpawn%20Area))) (Variables|Default|GetRotation%20Yaw))) "1,1,1"))
    (Utilities|Array|Add (Variables|FishSettings|GetInstanceAccelerationX) 0.0)
    (Utilities|Array|Add (Variables|FishSettings|GetInstanceAccelerationY) 0.0)
    (Utilities|Array|Add (Variables|FishSettings|GetInstanceVelocityX) 0.0)
    (Utilities|Array|Add (Variables|FishSettings|GetInstanceVelocityY) 0.0)))

(fn UpdateTroutInstances
  (params (DeltaTime :type Float%20%28single-precision%29))
  (bind _max_acceleration_x (Variables|FishSettings|GetMax%20Acceleration%20X))
  (bind _max__acceleration_y (Variables|Default|GetMax.%20Acceleration%20Y))
  (if (> (Utilities|Array|Length (Variables|FishSettings|GetFleeingTroutIndices)) 0)
    (Utilities|Array|Clear (LocalVariables|GetSaveTrouts))
    (Utilities|Array|Clear (LocalVariables|GetRemoveTrouts))
    (for _index (range (- 0 (Utilities|Array|LastIndex (Variables|FishSettings|GetFleeingTroutIndices))) 0)
      (LocalVariables|SetCurrentIndex (Utilities|Array|Get(acopy) (Variables|FishSettings|GetFleeingTroutIndices) (Math|Integer|Absolute(Integer) _index)))
      (LocalVariables|SetCurrentInstanceLocation (.location (.OutInstanceTransform (Components|InstancedStaticMesh|GetInstanceTransform (Variables|Components|GetInstancedStaticMesh) (LocalVariables|GetCurrentIndex) true))))
      (LocalVariables|SetCurrentInstanceRotation (.rotation (.OutInstanceTransform (Components|InstancedStaticMesh|GetInstanceTransform (Variables|Components|GetInstancedStaticMesh) (LocalVariables|GetCurrentIndex) true))))
      (bind _output_get (LocalVariables|SetCurrentInstanceScale (.scale (.OutInstanceTransform (Components|InstancedStaticMesh|GetInstanceTransform (Variables|Components|GetInstancedStaticMesh) (LocalVariables|GetCurrentIndex) true)))))
      (if (> (Math|Float|Clamp(Float) (- (Utilities|Array|Get(acopy) (Variables|FishSettings|GetInstanceAccelerationX) (LocalVariables|GetCurrentIndex)) (* DeltaTime (Variables|FishSettings|GetAcceleration%20Falloff))) (* -1.0 _max_acceleration_x) _max_acceleration_x) 0.0)
        (if (> (Utilities|Array|Get(acopy) (Variables|FishSettings|GetInstanceVelocityX) (LocalVariables|GetCurrentIndex)) 0.0)
          (LocalVariables|SetNewInstanceScale (LocalVariables|GetCurrentInstanceScale) :!label _label)
          (else
            (LocalVariables|SetNewInstanceScale (Utilities|PackInstanceScaleVector (LocalVariables|GetCurrentIndex) (Math|Float|Clamp(Float) (- (Utilities|Array|Get(acopy) (Variables|FishSettings|GetInstanceAccelerationX) (LocalVariables|GetCurrentIndex)) (* DeltaTime (Variables|FishSettings|GetAcceleration%20Falloff))) (* -1.0 _max_acceleration_x) _max_acceleration_x) (Math|Float|Clamp(Float) (- (Utilities|Array|Get(acopy) (Variables|FishSettings|GetInstanceAccelerationY) (LocalVariables|GetCurrentIndex)) (* DeltaTime (Variables|FishSettings|GetAcceleration%20Falloff))) (* -1.0 _max__acceleration_y) _max__acceleration_y)) :!label _label_2)))
        (elif (> (+ (Utilities|Array|Get(acopy) (Variables|FishSettings|GetInstanceVelocityX) (LocalVariables|GetCurrentIndex)) (* (Utilities|Array|Get(acopy) (Variables|FishSettings|GetInstanceAccelerationX) (LocalVariables|GetCurrentIndex)) DeltaTime)) 0.0)
          (if (> (.x _output_get) 1.0)
            (LocalVariables|SetCurrentInstanceRotation (Math|Rotator|CombineRotators (.rotation (.OutInstanceTransform (Components|InstancedStaticMesh|GetInstanceTransform (Variables|Components|GetInstancedStaticMesh) (LocalVariables|GetCurrentIndex) true))) (Math|Rotator|MakeRotator 0.0 0.0 (+ (Utilities|Array|Get(acopy) (Variables|FishSettings|GetInstanceVelocityY) (LocalVariables|GetCurrentIndex)) (* (Utilities|Array|Get(acopy) (Variables|FishSettings|GetInstanceAccelerationY) (LocalVariables|GetCurrentIndex)) DeltaTime)))))
            (goto _label_2)
            (else
              (goto _label)))
          (else
            (LocalVariables|SetNewInstanceScale "1.000000,1.000000,1.000000"))))
      (Components|InstancedStaticMesh|UpdateInstanceTransform (Variables|Components|GetInstancedStaticMesh) (LocalVariables|GetCurrentIndex) (Math|Transform|MakeTransform (+ (* (* (Math|Vector|GetForwardVector (LocalVariables|GetCurrentInstanceRotation)) (* (+ (Utilities|Array|Get(acopy) (Variables|FishSettings|GetInstanceVelocityX) (LocalVariables|GetCurrentIndex)) (* (Utilities|Array|Get(acopy) (Variables|FishSettings|GetInstanceAccelerationX) (LocalVariables|GetCurrentIndex)) DeltaTime)) 1.0)) -1) (LocalVariables|GetCurrentInstanceLocation)) (LocalVariables|GetCurrentInstanceRotation) (LocalVariables|GetNewInstanceScale)) true (== (Math|Integer|Absolute(Integer) _index) 0) false)
      (Utilities|Array|SetArrayElem (Variables|FishSettings|GetInstanceVelocityX) (LocalVariables|GetCurrentIndex) (* (+ (Utilities|Array|Get(acopy) (Variables|FishSettings|GetInstanceVelocityX) (LocalVariables|GetCurrentIndex)) (* (Utilities|Array|Get(acopy) (Variables|FishSettings|GetInstanceAccelerationX) (LocalVariables|GetCurrentIndex)) DeltaTime)) 1.0))
      (Utilities|Array|SetArrayElem (Variables|FishSettings|GetInstanceVelocityY) (LocalVariables|GetCurrentIndex) (+ (Utilities|Array|Get(acopy) (Variables|FishSettings|GetInstanceVelocityY) (LocalVariables|GetCurrentIndex)) (* (Utilities|Array|Get(acopy) (Variables|FishSettings|GetInstanceAccelerationY) (LocalVariables|GetCurrentIndex)) DeltaTime)))
      (if (> (Utilities|Array|Get(acopy) (Variables|FishSettings|GetInstanceVelocityX) (LocalVariables|GetCurrentIndex)) 0.0)
        (Utilities|Array|SetArrayElem (Variables|FishSettings|GetInstanceAccelerationX) (LocalVariables|GetCurrentIndex) (Math|Float|Clamp(Float) (- (Utilities|Array|Get(acopy) (Variables|FishSettings|GetInstanceAccelerationX) (LocalVariables|GetCurrentIndex)) (* DeltaTime (Variables|FishSettings|GetAcceleration%20Falloff))) (* -1.0 _max_acceleration_x) _max_acceleration_x))
        (Utilities|Array|SetArrayElem (Variables|FishSettings|GetInstanceAccelerationY) (LocalVariables|GetCurrentIndex) (Math|Float|Clamp(Float) (- (Utilities|Array|Get(acopy) (Variables|FishSettings|GetInstanceAccelerationY) (LocalVariables|GetCurrentIndex)) (* DeltaTime (Variables|FishSettings|GetAcceleration%20Falloff))) (* -1.0 _max__acceleration_y) _max__acceleration_y))
        (Utilities|Array|Add (LocalVariables|GetSaveTrouts) (LocalVariables|GetCurrentIndex))
        (else
          (Utilities|Array|SetArrayElem (Variables|FishSettings|GetInstanceVelocityX) (LocalVariables|GetCurrentIndex) 0.0)
          (Utilities|Array|SetArrayElem (Variables|FishSettings|GetInstanceVelocityY) (LocalVariables|GetCurrentIndex) 0.0)
          (Utilities|Array|SetArrayElem (Variables|FishSettings|GetInstanceAccelerationX) (LocalVariables|GetCurrentIndex) 0.0)
          (Utilities|Array|SetArrayElem (Variables|FishSettings|GetInstanceAccelerationY) (LocalVariables|GetCurrentIndex) 0.0))))
    (if (> (Utilities|Array|Length (LocalVariables|GetSaveTrouts)) 0)
      (Variables|FishSettings|SetFleeingTroutIndices (LocalVariables|GetSaveTrouts))
      (elif (> (Utilities|Array|Length (Variables|FishSettings|GetFleeingTroutIndices)) 0)
        (Utilities|Array|Clear (Variables|FishSettings|GetFleeingTroutIndices))))))

(fn GetInstanceCollisions
  (bind _instancedstaticmesh (Variables|Components|GetInstancedStaticMesh))
  (bind _troutawarenessradius (Variables|Default|GetTroutAwarenessRadius))
  (bind _nexttracelocation (Variables|FishSettings|GetNextTraceLocation))
  (bind _nexttracelocation_2 (Variables|FishSettings|GetNextTraceLocation))
  (bind _returnvalue (Utilities|Array|LastIndex _nexttracelocation))
  (bind _output (Utilities|Array|Get(acopy) _nexttracelocation _returnvalue))
  (bind _returnvalue_2 (Class|InstancedStaticMeshComponent|GetInstancesOverlappingSphere _instancedstaticmesh _output _troutawarenessradius true))
  (if (Variables|Default|GetTraceOnNext)
    (if (> (Utilities|Array|Length _returnvalue_2) 0)
      (for _array_element _returnvalue_2
        (Utilities|Array|SetArrayElem (Variables|FishSettings|GetInstanceAccelerationX) _array_element (Variables|FishSettings|GetMax%20Acceleration%20X))
        (bind _returnvalue_3 (Utilities|Array|AddUnique (Variables|FishSettings|GetFleeingTroutIndices) _array_element))
        (if (== _returnvalue_3 -1)
          _)))
    (Utilities|Array|RemoveIndex _nexttracelocation_2 _returnvalue)
    (if (not (> (Utilities|Array|Length _nexttracelocation_2) 0))
      (Variables|Default|SetTraceOnNext false))))

(fn SetTraceLocation
  (params (Location :type Vector) (Radius :type Float%20%28single-precision%29))
  (Utilities|Array|AddUnique (Variables|FishSettings|GetNextTraceLocation) Location)
  (Utilities|Array|Add (Variables|FishSettings|GetNextTraceRadius) Radius)
  (Variables|Default|SetTraceOnNext true))

(fn SetNewTarget
  (params (NewTarget :type Vector))
  (Utilities|Array|AddUnique (Variables|Targets|GetTargetLocations) NewTarget))

(fn RemoveTarget
  (params (TargetIndex :type Integer))
  (Utilities|Array|RemoveIndex (Variables|Targets|GetTargetLocations) TargetIndex))

(fn SetNewSurfaceTarget
  (params (NewTarget :type Vector))
  (bind (_x _y) (Math|Vector|BreakVector NewTarget))
  (Targets|SetNewTarget (Math|Vector|MakeVector _x _y (Variables|WaterInfo|GetWaterHeight))))