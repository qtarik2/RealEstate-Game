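; BP_BeefyFlightPointActor is a placeable waypoint that marks one ordered point on a numbered AI flight path.
; It writes its FlightPathIndex into its actor tags, letting points on the same path find each other.
; In construction and at BeginPlay, an unset Order becomes one above the path's highest; construction also reassigns out-of-range orders.
; GetRandomPathOffset returns a seed-repeatable offset scaled by RandomHeight, plus that maximum.
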(event EventBeginPlay
  (CallFunction|SetFlightPathIndexTag)
  (if (== (Variables|Default|GetOrder) -1)
    (CallFunction|SetOrder)))

(event Collision|EventActorBeginOverlap
  (params (OtherActor :type Actor%20Object%20Reference)))

(event EventTick
  (params (DeltaSeconds :type Float%20%28single-precision%29)))

(fn ConstructionScript
  (bind _order (Variables|Default|GetOrder))
  (CallFunction|SetFlightPathIndexTag)
  (bind _outactors (Actor|GetAllActorsOfClasswithTag "BP_BeefyFlightPointActor_C" (Utilities|String|StringToName (Utilities|String|ToString(Integer) (Variables|Default|GetFlightPathIndex)))))
  (if (or (== _order -1) (> _order (Utilities|Array|LastIndex _outactors)))
    (CallFunction|SetOrder)))

(fn SetFlightPathIndexTag
  (Utilities|Array|Add (LocalVariables|GetNewFlightPathIndexTag) (Utilities|String|StringToName (Utilities|String|ToString(Integer) (Variables|Default|GetFlightPathIndex))))
  (Variables|Default|SetTags (LocalVariables|GetNewFlightPathIndexTag)))

(fn SetOrder
  (bind _outactors (Actor|GetAllActorsOfClasswithTag "BP_BeefyFlightPointActor_C" (Utilities|String|StringToName (Utilities|String|ToString(Integer) (Variables|Default|GetFlightPathIndex)))))
  (LocalVariables|SetSceneFlightPathActors _outactors)
  (LocalVariables|SetHighestOrder -1)
  (for _array_element (LocalVariables|GetSceneFlightPathActors)
    (bind _asbp_beefy_flight_point_actor (Utilities|Casting|CastToBP_BeefyFlightPointActor _array_element))
    (if (> (Variables|BP_BeefyFlightPointActor_C|GetOrder _asbp_beefy_flight_point_actor) (LocalVariables|GetHighestOrder))
      (LocalVariables|SetHighestOrder (Variables|BP_BeefyFlightPointActor_C|GetOrder _asbp_beefy_flight_point_actor))))
  (Variables|Default|SetOrder (+ (LocalVariables|GetHighestOrder) 1)))

(fn GetRandomPathOffset
  (params (Seed :type Integer))
  (return (* (Variables|Default|GetRandomHeight) (Math|Random|RandomFloatfromStream (Math|Random|MakeRandomStream Seed))) (Variables|Default|GetRandomHeight)))