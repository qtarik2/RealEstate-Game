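; BP_Projectile is a physics-configurable projectile that sets up Beefy grass and interaction components.
; Its construction script scales the collision by projectile size and toggles custom depth stencil for cel shading.
; It passes the particle system to the grass component, and the collision, wake/idle timing, buoyancy and physics settings to the interaction component.
; SpawnParticle emits dust clouds at the hit location, throttled by a spawn interval.
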(fn ConstructionScript
  (CallFunction|SetProjectileSize (Variables|Default|GetProjectileSize))
  (if (Variables|Default|GetCelShading)
    (Rendering|SetRenderCustomDepth (Variables|Default|GetStaticMesh) true)
    (Rendering|SetCustomDepthStencilValue (Variables|Default|GetStaticMesh) 1)
    (else
      (Rendering|SetRenderCustomDepth (Variables|Default|GetStaticMesh) false)))
  (Default|Initialize (Variables|Default|GetBP_BeefyGrassComponent) (Utilities|Array|MakeArray (Variables|Default|GetParticleSystem)))
  ;[1 1 1] Interaction Component Setup
  (Default|InitializeComponent (Variables|Default|GetBP_BeefyInteractionComponent) (Variables|Default|GetStaticMeshCollision) (Variables|Default|GetTimeInterval) (Variables|Default|GetWakeTimeInterval) (Variables|Default|GetIdleTimeInterval) (Variables|Default|GetWakeSpeedLimit) (Variables|Default|GetBuoyantMass) true (Variables|Default|GetEnablePhysics)))

(fn SetProjectileSize
  (params (Size :type Float%20%28single-precision%29))
  (Transformation|SetRelativeScale3D (Variables|Default|GetStaticMeshCollision) (Math|Conversions|ToVector(Float) Size)))

(fn SpawnParticle
  (if (>= (- (Utilities|Time|GetGameTimeinSeconds) (Variables|Default|GetTimeOfLastParticleSpawn)) (Variables|Default|GetSpawnInterval))
    (Variables|Default|SetTimeOfLastParticleSpawn (Utilities|Time|GetGameTimeinSeconds))
    (Effects|SpawnEmitteratLocation "/Game/BeefyGrassLands/Blueprints/FootPrintBP/Particles/P_DustClouds.P_DustClouds" (Variables|Default|GetHitLocation))))