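; Water interaction component that gives a collision component wake, idle and splash effects plus optional simple buoyancy in water.
; Entering or waking starts a looping timer, used instead of Tick, that spawns foam-tinted particles by speed and applies forces.
; Surface height and rotation come from the closest spline point, or the water component's transform otherwise.
; Physics mode swaps gravity for box-bounds buoyancy, current push and water damping until exit.
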(event EventBeginPlay
  (Variables|Default|SetLastLocation (Transformation|GetWorldLocation)))

(event EventTick
  (params (DeltaSeconds :type Float%20%28single-precision%29)))

(fn StartWading
  (if (not (Variables|Default|GetTimerEnabled))
    (Variables|Default|SetLastLocation (Transformation|GetWorldLocation))
    (bind _returnvalue (Utilities|Time|SetTimerbyFunctionName 0 "ParticleTimerUpdate" (Variables|Default|GetTimeInterval) true))
    (Variables|Default|SetTimerHandle _returnvalue)
    (Variables|Default|SetTimerEnabled true)))

(fn ParticleTimerUpdate
  (bind _returnvalue (Transformation|GetWorldLocation))
  (LocalVariables|SetSpeed (+ (/ (Math|Vector|VectorLength (- (Transformation|GetWorldLocation) (Variables|Default|GetLastLocation))) (- (Utilities|Time|GetGameTimeinSeconds) (Variables|Default|GetTimeOfLastMovement))) 1e-05))
  (LocalVariables|SetScalingWakeTimeInterval (* (/ 1.0 (Math|Float|Clamp(Float) (/ (LocalVariables|GetSpeed) (Variables|Default|GetMaxSpeed)))) (Variables|Default|GetWakeTimeInterval)))
  (bind (_worldheight _splinerotation) (Particles|GetWaterMeshHeight (Variables|Default|GetLastLocation)))
  (LocalVariables|SetParticleHeight _worldheight)
  (LocalVariables|SetParticleRotation _splinerotation)
  (if (and (< (Math|Float|Absolute(Float) (- _worldheight (.Z (Math|Vector|BreakVector (Variables|Default|GetLastLocation))))) (Variables|Default|GetCollisionRadius)) (> (LocalVariables|GetSpeed) (Variables|Default|GetWakeSpeedLimit)))
    (Variables|Default|SetLastLocation (Transformation|GetWorldLocation))
    (if (>= (- (Utilities|Time|GetGameTimeinSeconds) (Variables|Default|GetTimeOfLastMovement)) (LocalVariables|GetScalingWakeTimeInterval))
      (LocalVariables|SetNewParticle (Variables|Default|GetWakeParticle))
      (Variables|Default|SetTimeOfLastMovement (Utilities|Time|GetGameTimeinSeconds) :!label _label)
      (Particles|SpawnParticle (LocalVariables|GetNewParticle) (Math|Vector|MakeVector (.x _returnvalue) (.y _returnvalue) (LocalVariables|GetParticleHeight)) (LocalVariables|GetParticleRotation)))
    (elif (and (< (Math|Float|Absolute(Float) (- _worldheight (.Z (Math|Vector|BreakVector (Variables|Default|GetLastLocation))))) (Variables|Default|GetCollisionRadius)) (not (> (LocalVariables|GetSpeed) (Variables|Default|GetWakeSpeedLimit))))
      (if (> (- (Utilities|Time|GetGameTimeinSeconds) (Variables|Default|GetTimeOfLastMovement)) (- (Variables|Default|GetIdleTimeInterval) 0.02))
        (LocalVariables|SetNewParticle (Variables|Default|GetIdleParticle))
        (goto _label)
        (else
          _))
      (else
        (Variables|Default|SetTimeOfLastMovement (Utilities|Time|GetGameTimeinSeconds))
        (Variables|Default|SetLastLocation (Transformation|GetWorldLocation)))))
  (Interaction|ApplyForces))

(fn StopWading
  (if (Variables|Default|GetTimerEnabled)
    (Utilities|Time|ClearandInvalidateTimerbyHandle (Variables|Default|GetTimerHandle))
    (Variables|Default|SetTimerEnabled false)))

(fn SetWaterParameters
  (params (WaterComponent :type Scene%20Component%20Object%20Reference) (ParticleColor :type Color%20Structure) (WaterSpeed :type Float%20%28single-precision%29))
  (Variables|Default|SetWaterComponent WaterComponent)
  (Variables|Default|SetFoamColor ParticleColor)
  (Variables|Default|SetWaterSpeed WaterSpeed))

(fn InitializeComponent
  (params (Collision :type Primitive%20Component%20Object%20Reference) (TimeInterval :type Float%20%28single-precision%29) (WakeTimeInterval :type Float%20%28single-precision%29) (IdleTimeInterval :type Float%20%28single-precision%29) (WakeSpeedLimit :type Float%20%28single-precision%29) (BuoyantMass :type Float%20%28single-precision%29) (WakeOnBegin :type Boolean) (ApplyPhysics :type Boolean) (Debug :type Boolean))
  (Variables|Default|SetCollisionComponent Collision)
  (Setup|UpdateComponentBounds)
  (Variables|Default|SetTimeInterval TimeInterval)
  (Variables|Default|SetWakeSpeedLimit WakeSpeedLimit)
  (Variables|Default|SetWakeTimeInterval WakeTimeInterval)
  (Variables|Default|SetIdleTimeInterval IdleTimeInterval)
  (Variables|Default|SetBuoyantMass BuoyantMass)
  (Variables|Default|SetWakeOnBegin WakeOnBegin)
  (Variables|Default|SetPhysicsEnabled ApplyPhysics)
  (Variables|Default|SetDebug Debug))

(fn WakeUp
  (params (WaterComponent :type Scene%20Component%20Object%20Reference) (ParticleColor :type Color%20Structure) (Random :type Float%20%28single-precision%29) (WaterSpeed :type Float%20%28single-precision%29))
  (if (not (Variables|Default|GetTimerEnabled))
    (Setup|SetWaterParameters WaterComponent ParticleColor WaterSpeed)
    (Variables|Default|SetLastLocation (Transformation|GetWorldLocation))
    (Utilities|Time|SetTimerbyFunctionName self "StartWading" (* Random (Math|Random|RandomFloat)))))

(fn SetParticles
  (params (Wake :type Particle%20System%20Object%20Reference) (Idle :type Particle%20System%20Object%20Reference) (Splash :type Particle%20System%20Object%20Reference))
  (Variables|Default|SetWakeParticle Wake)
  (Variables|Default|SetIdleParticle Idle)
  (Variables|Default|SetSplashParticle Splash))

(fn SpawnParticleNearLocation
  (params (Location :type Vector) (Particle :type Particle%20System%20Object%20Reference))
  (bind (_worldheight _splinerotation) (Particles|GetWaterMeshHeight Location))
  (LocalVariables|SetHeight _worldheight)
  (Particles|SpawnParticle Particle (Math|Vector|MakeVector (.x Location) (.y Location) (LocalVariables|GetHeight)) _splinerotation))

(fn EnterWater
  (params (WaterComponent :type Scene%20Component%20Object%20Reference) (ParticleColor :type Color%20Structure) (WaterSpeed :type Float%20%28single-precision%29))
  (Setup|SetWaterParameters WaterComponent ParticleColor WaterSpeed)
  (if (> (Math|Float|Absolute(Float) (.z (Transformation|GetComponentVelocity (Variables|Default|GetCollisionComponent)))) (Variables|Default|GetSplashSpeedZ))
    (LocalVariables|SetNewParticle (Variables|Default|GetSplashParticle))
    (else
      (LocalVariables|SetNewParticle (Variables|Default|GetWakeParticle))))
  (Particles|SpawnParticleNearLocation (Transformation|GetWorldLocation) (LocalVariables|GetNewParticle))
  (Interaction|StartWading)
  (Interaction|HandlePhysics))

(fn ExitWater
  (if (Variables|Default|GetTimerEnabled)
    (if (> (Math|Float|Absolute(Float) (.z (Transformation|GetComponentVelocity (Variables|Default|GetCollisionComponent)))) (Variables|Default|GetSplashSpeedZ))
      (LocalVariables|SetNewParticle (Variables|Default|GetSplashParticle))
      (else
        (LocalVariables|SetNewParticle (Variables|Default|GetWakeParticle))))
    (Particles|SpawnParticleNearLocation (Transformation|GetWorldLocation) (Variables|Default|GetWakeParticle))
    (Interaction|StopWading)
    (Interaction|HandlePhysics)))

(fn StartWadingImmediately
  (if (not (Variables|Default|GetTimerEnabled))
    (Particles|ParticleTimerUpdate)
    (Interaction|StartWading)))

(fn WakeUponBegin
  (params (WaterComponent :type Scene%20Component%20Object%20Reference) (ParticleColor :type Color%20Structure) (Random :type Float%20%28single-precision%29) (WaterSpeed :type Float%20%28single-precision%29))
  (if (Variables|Default|GetWakeOnBegin)
    (Setup|WakeUp WaterComponent ParticleColor Random WaterSpeed)
    (else
      (Setup|SetWaterParameters WaterComponent ParticleColor WaterSpeed))))

(fn GetWaterMeshHeight
  (params (Location :type Vector))
  (bind _asspline_component (Utilities|Casting|CastToSplineComponent (Variables|Default|GetWaterComponent))
    (:then
      (LocalVariables|SetHeight (.z (Spline|FindLocationClosesttoWorldLocation _asspline_component Location "World")))
      (LocalVariables|SetRotation (Math|Rotator|MakeRotationfromAxes (Spline|FindDirectionClosesttoWorldLocation _asspline_component Location "World") (Math|Vector|CrossProduct (Class|SplineComponent|FindUpVectorClosesttoWorldLocation _asspline_component Location "World") (Spline|FindDirectionClosesttoWorldLocation _asspline_component Location "World")) (Class|SplineComponent|FindUpVectorClosesttoWorldLocation _asspline_component Location "World"))))
    (:CastFailed
      (LocalVariables|SetHeight (.z (Transformation|GetWorldLocation (Variables|Default|GetWaterComponent))))
      (LocalVariables|SetRotation (Transformation|GetWorldRotation (Variables|Default|GetWaterComponent)))))
  (return (LocalVariables|GetHeight) (LocalVariables|GetRotation)))

(fn SpawnParticle
  (params (Particle :type Particle%20System%20Object%20Reference) (Location :type Vector) (Rotation :type Rotator))
  (bind _returnvalue (Effects|SpawnEmitteratLocation Particle Location Rotation))
  (Rendering|SetTranslucentSortPriority _returnvalue 10)
  (Effects|Components|ParticleSystem|SetColorParameter _returnvalue "Foam Color" (Math|Conversions|ToLinearColor(Color) (Variables|Default|GetFoamColor)))
  (Effects|Components|ParticleSystem|SetFloatParameter _returnvalue "WaterSpeed" (Variables|Default|GetWaterSpeed)))

(fn SetParticleComponent
  (params (NewParticleComponent :type Particle%20System%20Component%20Object%20Reference))
  (Variables|Default|SetParticleComponent NewParticleComponent))

(fn HandlePhysics
  (if (and (Variables|Default|GetPhysicsEnabled) (Physics|IsSimulatingPhysics (Variables|Default|GetCollisionComponent) "None"))
    (if (Variables|Default|GetTimerEnabled)
      (Physics|SetEnableGravity (Variables|Default|GetCollisionComponent) false)
      (Variables|Default|SetSavedDampenValue (Class|PrimitiveComponent|GetLinearDamping (Variables|Default|GetCollisionComponent)))
      (Class|PrimitiveComponent|SetLinearDamping (Variables|Default|GetCollisionComponent) (Variables|Default|GetWaterFriction))
      (else
        (Physics|SetEnableGravity (Variables|Default|GetCollisionComponent) true)
        (Class|PrimitiveComponent|SetLinearDamping (Variables|Default|GetCollisionComponent) (Variables|Default|GetSavedDampenValue))))))

(fn ApplyForces
  (bind _collisioncomponent (Variables|Default|GetCollisionComponent))
  (bind (_origin _boxextent) (Collision|GetComponentBounds _collisioncomponent))
  (bind _returnvalue (/ (.z _boxextent) 1e+02))
  (if (and (Variables|Default|GetPhysicsEnabled) (Physics|IsSimulatingPhysics (Variables|Default|GetCollisionComponent) "None"))
    (bind (_worldheight _splinerotation) (Particles|GetWaterMeshHeight _origin))
    (Physics|AddForce (Variables|Default|GetCollisionComponent) (* (+ (* (Math|Rotator|GetRotationXVector _splinerotation) (Variables|Default|GetWaterSpeed)) (* "0, 0,1.000000" (* (Math|Float|Clamp(Float) (/ 1.0 (Variables|Default|GetBuoyantMass)) 1.0 1e+01) (+ (* (* (Math|Float|Clamp(Float) (- (/ _worldheight 1e+02) (- (/ (.Z (Math|Vector|BreakVector _origin)) 1e+02) (/ _returnvalue 2.0))) 0.0 _returnvalue) (/ (.x _boxextent) 1e+02) (/ (.y _boxextent) 1e+02)) 9.8e+03) (* (Variables|Default|GetBuoyantMass) -9.8))))) (Variables|Default|GetForce%20Multiplier)) "None" true)))

(fn UpdateComponentBounds
  (Variables|Default|SetCollisionRadius (.SphereRadius (Collision|GetComponentBounds (Variables|Default|GetCollisionComponent)))))