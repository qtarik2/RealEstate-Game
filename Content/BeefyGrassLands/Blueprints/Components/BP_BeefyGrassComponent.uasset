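; Grass interaction component that lets its owner disturb grass through a scene-captured vector field.
; Registers configured particle components, a background plane and spawned footprint, impact and fade-out emitters with the level's first BP_GrassVectorFieldCapture, found on demand.
; Also spawns visible grass footprint effects, harvests foliage ISM instances overlapping its collision component, and line-traces to place surface-aligned BP_GrassOccluder actors for distance field culling.
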(event EventBeginPlay
  (Main|AddComponentstoVectorField))

(fn AddComponentstoVectorField
  (Utilities|IsValid (Variables|Default|GetVectorFieldSceneCaptureBP)
    (:Is%20Valid
      _)
    (:Is%20Not%20Valid
      (Main|GetVectorFieldSceneCapture)
      (Utilities|IsValid (Variables|Default|GetVectorFieldSceneCaptureBP)
        (:Is%20Valid
          _))))
  (for _array_element (Variables|Default|GetVectorFieldComponents)
    (LocalVariables|SetComp _array_element)
    (Default|AddtoSceneCaptureList (Variables|Default|GetVectorFieldSceneCaptureBP) (LocalVariables|GetComp))))

(fn AddSingleComponenttoVectorField
  (params (Comp :type Primitive%20Component%20Object%20Reference))
  (Utilities|IsValid (Variables|Default|GetVectorFieldSceneCaptureBP)
    (:Is%20Valid
      _)
    (:Is%20Not%20Valid
      (Main|GetVectorFieldSceneCapture)
      (Utilities|IsValid (Variables|Default|GetVectorFieldSceneCaptureBP)
        (:Is%20Valid
          _))))
  (Default|AddtoSceneCaptureList (Variables|Default|GetVectorFieldSceneCaptureBP) Comp))

(fn Initialize
  (params (Components :type Array%20of%20Primitive%20Component%20Object%20References) (Collision :type Sphere%20Component%20Object%20Reference))
  (Variables|Default|SetVectorFieldComponents Components)
  (Variables|Default|SetFoliageCollision Collision)
  (for _array_element Components
    (LocalVariables|SetComp _array_element)
    (Transformation|SetAbsolute (LocalVariables|GetComp) false true false)
    (Main|AddComponentstoVectorField)
    (bind _asparticle_system_component (Utilities|Casting|CastToParticleSystemComponent (LocalVariables|GetComp)))
    (Effects|Components|ParticleSystem|SetTemplate _asparticle_system_component (Variables|Default|GetVectorFieldParticle))
    (Effects|Components|ParticleSystem|SetFloatParameter _asparticle_system_component "Size" (Variables|Default|GetFootParticleSize))))

(fn SetBackgroundPlane
  (params (Mesh :type Static%20Mesh%20Component%20Object%20Reference))
  (Components|StaticMesh|SetStaticMesh Mesh "/Engine/BasicShapes/Plane.Plane")
  (Transformation|SetRelativeTransform Mesh (Math|Transform|MakeTransform "0, 0,-5000.000000" "0, 0, 0" "1000.000000,1000.000000,1") false false)
  (Class|PrimitiveComponent|SetOwnerNoSee Mesh false)
  (Rendering|SetCastShadow Mesh false)
  (Collision|SetCollisionEnabled Mesh "NoCollision")
  (Rendering|Material|SetMaterial Mesh 0 "/Game/BeefyGrassLands/RenderTargetBP/Materials/M_VectorFieldBackground.M_VectorFieldBackground")
  (Transformation|SetAbsolute Mesh false true false)
  (Utilities|Array|AddUnique (Variables|Default|GetVectorFieldComponents) Mesh))

(fn GetVectorFieldSceneCapture
  (bind _outactors (Actor|GetAllActorsOfClass "/Game/BeefyGrassLands/RenderTargetBP/BP_GrassVectorFieldCapture.BP_GrassVectorFieldCapture_C"))
  (if (Utilities|Array|IsValidIndex _outactors)
    (bind _output_get (Variables|Default|SetVectorFieldSceneCaptureBP (Utilities|Array|Get(acopy) _outactors)))
    (return _output_get)))

(fn SpawnVectorFieldFootPrintParticle
  (params (NewLocation :type Vector))
  (bind _returnvalue (Effects|SpawnEmitteratLocation (Variables|Default|GetVectorFieldFootPrintParticle) NewLocation))
  (bind _output_get (LocalVariables|SetNewEmitter _returnvalue))
  (Effects|Components|ParticleSystem|SetFloatParameter _output_get "Size" (Variables|Default|GetFootParticleSize))
  (Rendering|SetTranslucentSortPriority (LocalVariables|GetNewEmitter) 1)
  (Main|AddSingleComponenttoVectorField (LocalVariables|GetNewEmitter)))

(fn SpawnGrassFootPrintParticle
  (params (NewLocation :type Vector))
  (bind _returnvalue (Effects|SpawnEmitteratLocation (Variables|Default|GetGrassFootPrintParticleEffect) NewLocation))
  (LocalVariables|SetNewEmitter _returnvalue))

(fn HarvestFoliageISM
  (for _array_element (Class|PrimitiveComponent|GetOverlappingComponents (Variables|Default|GetFoliageCollision))
    (bind _asbp_beefy_foliage_ism_master (Utilities|Casting|CastToBP_BeefyFoliageISM_Master _array_element))
    (Default|HarvestNearbyInstances _asbp_beefy_foliage_ism_master (Variables|Default|GetFoliageCollision))))

(fn SpawnVectorFieldImpactParticle
  (bind _returnvalue (Effects|SpawnEmitteratLocation "/Game/BeefyGrassLands/RenderTargetBP/Particles/P_VectorFieldParticle_Impact.P_VectorFieldParticle_Impact" (Transformation|GetWorldLocation (Variables|Default|GetFoliageCollision))))
  (LocalVariables|SetNewEmitter _returnvalue)
  (Rendering|SetTranslucentSortPriority (LocalVariables|GetNewEmitter) 10)
  (Effects|Components|ParticleSystem|SetFloatParameter (LocalVariables|GetNewEmitter) "Size" (Variables|Default|GetImpactParticleSize))
  (Main|AddSingleComponenttoVectorField (LocalVariables|GetNewEmitter)))

(fn SpawnDistanceFieldCullingActor
  (bind _foliagecollision (Variables|Default|GetFoliageCollision))
  (bind _returnvalue (Transformation|GetWorldLocation _foliagecollision))
  (bind (_outhit _returnvalue_2) (Collision|LineTraceByChannel _returnvalue (+ _returnvalue (Math|Vector|MakeVector 0.0 0.0 (Variables|Default|GetTraceDepth))) "TraceTypeQuery1" false 0 "None"))
  (if _returnvalue_2
    (Game|SpawnActorfromClass "/Game/BeefyGrassLands/Blueprints/Foliage/BP_GrassOccluder.BP_GrassOccluder_C" (Math|Transform|MakeTransform (.location _outhit) (Math|Rotator|MakeRotfromZ (.normal _outhit)) "1,1,1") "Undefined" 0 0)))

(fn SpawnVectorFieldFadeOutParticle
  (params (NewLocation :type Vector))
  (bind _returnvalue (Effects|SpawnEmitteratLocation (Variables|Default|GetVectorFieldFadeOutParticle) NewLocation))
  (bind _output_get (LocalVariables|SetNewEmitter _returnvalue))
  (Effects|Components|ParticleSystem|SetFloatParameter _output_get "Size" (Variables|Default|GetFootParticleSize))
  (Rendering|SetTranslucentSortPriority (LocalVariables|GetNewEmitter) 1)
  (Main|AddSingleComponenttoVectorField (LocalVariables|GetNewEmitter)))