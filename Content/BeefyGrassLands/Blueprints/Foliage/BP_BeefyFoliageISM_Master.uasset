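; Master foliage instanced-mesh Blueprint for harvestable plants that can be picked within a sphere, with helpers for random item drops.
; Picking records each instance's index, scale and time, then rewrites its scale through PackInstanceAnimScale, apparently encoding animation timing for the material.
; A self-rescheduling timer resets harvested batches in order once ResetTime elapses.
; PickFlowerOnly is passed to the material as custom primitive data and selects the reset scale.
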(event EventBeginPlay
  (Main|SetCustomPrimitiveData (Variables|Main|GetPickFlowerOnly)))

(event EventTick
  (params (DeltaSeconds :type Float%20%28single-precision%29)))

(fn GetHarvestInfo
  (return (Variables|Harvest|GetFlowerStalkCount) (Variables|Main|GetPickFlowerMesh)))

(fn SpawnItems
  (params (NewLocation :type Vector))
  (bind _indices (Drops|GetRandomItemIndices))
  (for _array_element _indices
    (Game|SpawnActorfromClass (Utilities|Array|Get(acopy) (Variables|Drops|GetDropActors) _array_element) (Math|Transform|MakeTransform NewLocation (Math|Random|RandomRotator false) "1,1,1") "Undefined" 0 0)))

(fn GetRandomItemIndices
  (LocalVariables|SetRandom (Math|Random|RandomFloat))
  (for (_array_element _array_index) (Variables|Drops|GetDropRates)
    (if (<= (LocalVariables|GetRandom) _array_element)
      (Utilities|Array|Add (LocalVariables|GetDropIndices) _array_index)))
  (return (LocalVariables|GetDropIndices)))

(fn PickInstance
  (params (Index :type Integer) (LastIndex :type Boolean))
  (bind _pickedinstanceindicesmap (Variables|Harvest|GetPickedInstanceIndicesMap))
  (bind (_value _returnvalue) (Utilities|Map|Find _pickedinstanceindicesmap Index))
  (LocalVariables|SetInstanceTransform (.OutInstanceTransform (Components|InstancedStaticMesh|GetInstanceTransform Index true)))
  (LocalVariables|SetisAvailable (or (== _value 0) (not _returnvalue)))
  (if (LocalVariables|GetisAvailable)
    (Utilities|Array|Add (Variables|Harvest|GetHarvestedIndices) Index)
    (Utilities|Map|Add (Variables|Harvest|GetPickedInstanceScalesMap) Index (.scale (LocalVariables|GetInstanceTransform)))
    (Utilities|Map|Add (Variables|Harvest|GetPickedInstanceTimesMap) Index (Utilities|Time|GetGameTimeinSeconds))
    (Utilities|Map|Add (Variables|Harvest|GetPickedInstanceIndicesMap) Index 1)
    (Components|InstancedStaticMesh|UpdateInstanceTransform Index (Math|Transform|MakeTransform (.location (LocalVariables|GetInstanceTransform)) (.rotation (LocalVariables|GetInstanceTransform)) (Utilities|PackInstanceAnimScale Index 1.0)) true LastIndex false)
    (return (LocalVariables|GetisAvailable))
    (elif LastIndex
      (Components|InstancedStaticMesh|UpdateInstanceTransform Index (LocalVariables|GetInstanceTransform) true true false)
      (return (LocalVariables|GetisAvailable)))))

(fn HarvestNearbyInstances
  (params (Sphere :type Sphere%20Component%20Object%20Reference))
  (bind _output_get (LocalVariables|SetoverlappingInstances (Class|InstancedStaticMeshComponent|GetInstancesOverlappingSphere (Transformation|GetWorldLocation Sphere) (Variables|/Script/Engine.SphereComponent|GetSphereRadius Sphere) true)))
  (for (_array_element _array_index) _output_get
    (bind _output_get_2 (LocalVariables|SetcurrentIndex _array_element))
    (bind _waspicked (Harvest|PickInstance _output_get_2 (== _array_index (Utilities|Array|LastIndex (LocalVariables|GetoverlappingInstances)))))
    (if _waspicked
      (Math|Integer|IncrementInt (LocalVariables|GetharvestTotal))))
  (Utilities|Array|Add (Variables|Harvest|GetHarvestTotals) (LocalVariables|GetharvestTotal))
  (if (not (Variables|Main|GetSpawnTimerSet))
    (Variables|Main|SetSpawnTimerSet true)
    (Utilities|Time|SetTimerbyFunctionName 0 "ResetFoliage" (Variables|Main|GetResetTime)))
  (return (LocalVariables|GetharvestTotal)))

(fn SpawnParticle
  (params (Template :type Particle%20System%20Object%20Reference) (Location :type Vector) (Rotation :type Rotator) (Scale :type Float%20%28single-precision%29))
  (bind _returnvalue (Effects|SpawnEmitteratLocation Template Location Rotation))
  (LocalVariables|SetNewParticle _returnvalue))

(fn ResetFoliage
  (if (Utilities|Array|IsValidIndex (Variables|Harvest|GetHarvestTotals))
    (for _index (range 0 (- (Utilities|Array|Get(acopy) (Variables|Harvest|GetHarvestTotals)) 1))
      (bind _waspicked (Harvest|ResetInstance (Utilities|Array|Get(acopy) (Variables|Harvest|GetHarvestedIndices) (- (- (Utilities|Array|Get(acopy) (Variables|Harvest|GetHarvestTotals)) 1) _index)) (== (- (- (Utilities|Array|Get(acopy) (Variables|Harvest|GetHarvestTotals)) 1) _index) 0)))
      (if _waspicked
        (Utilities|Array|RemoveIndex (Variables|Harvest|GetHarvestedIndices) (- (- (Utilities|Array|Get(acopy) (Variables|Harvest|GetHarvestTotals)) 1) _index))
        (else
          (LocalVariables|SetCalledTooEarly true))))
    (if (Utilities|Array|IsValidIndex (Variables|Harvest|GetHarvestedIndices))
      (bind _output_get (LocalVariables|SetNewTimerWait (- (+ (.Value (Utilities|Map|Find (Variables|Harvest|GetPickedInstanceTimesMap) (Utilities|Array|Get(acopy) (Variables|Harvest|GetHarvestedIndices)))) (Variables|Main|GetResetTime)) (Utilities|Time|GetGameTimeinSeconds))))
      (if (<= _output_get 0.0)
        (LocalVariables|SetNewTimerWait 0.02))
      (Utilities|Time|SetTimerbyFunctionName 0 "ResetFoliage" (LocalVariables|GetNewTimerWait))
      (else
        (Variables|Main|SetSpawnTimerSet false)))
    (if (not (LocalVariables|GetCalledTooEarly))
      (Utilities|Array|RemoveIndex (Variables|Harvest|GetHarvestTotals)))))

(fn ResetInstance
  (params (Index :type Integer) (markDirty :type Boolean))
  (bind _pickedinstancescalesmap (Variables|Harvest|GetPickedInstanceScalesMap))
  (bind _outinstancetransform (Components|InstancedStaticMesh|GetInstanceTransform Index true))
  (bind (_value _returnvalue) (Utilities|Map|Find _pickedinstancescalesmap Index))
  (if _returnvalue
    (LocalVariables|SetPickedInstanceScale _value)
    (bind _output_get (LocalVariables|SetTimeIsRipe (>= (Utilities|Time|GetGameTimeinSeconds) (+ (.Value (Utilities|Map|Find (Variables|Harvest|GetPickedInstanceTimesMap) Index)) (Variables|Main|GetResetTime)))))
    (if _output_get
      (if (Variables|Main|GetPickFlowerOnly)
        (LocalVariables|SetInstanceScale (+ (LocalVariables|GetPickedInstanceScale) "0, 0,-0.100000"))
        (else
          (LocalVariables|SetInstanceScale "0, 0, 0")))
      (Components|InstancedStaticMesh|UpdateInstanceTransform Index (Math|Transform|MakeTransform (.location _outinstancetransform) (.rotation _outinstancetransform) (LocalVariables|GetInstanceScale)) true markDirty false))
    (return (LocalVariables|GetTimeIsRipe))))

(fn SetCustomPrimitiveData
  (params (PickFlowerOnly :type Boolean))
  (Rendering|Material|SetCustomPrimitiveDataFloat 8 (Math|Conversions|ToFloat(Boolean) PickFlowerOnly)))