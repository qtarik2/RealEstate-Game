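; Grass occluder that grows a disk mesh (DFDisk) outward from zero width, apparently to clear or mask grass around it.
; Construction collapses the disk in X and Y; BeginPlay starts a delayed looping timer.
; UpdateMesh lerps XY scale to the final size over the animation time, then clears the timer.
; A separate helper counts grass mesh instances overlapping the disk's bounding sphere.
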(event EventBeginPlay
  (bind _returnvalue (Utilities|Time|SetTimerbyFunctionName 0 "UpdateMesh" (Variables|Default|GetUpdateInterval) true (Variables|Default|GetSpawnDelay)))
  (Variables|Default|SetTimerHandle _returnvalue))

(fn ConstructionScript
  (Transformation|SetWorldScale3D (Variables|Default|GetDFDisk) (Math|Vector|MakeVector 0.0 0.0 1.0)))

(fn GetOverlappingFoliageCount
  (bind _dfdisk (Variables|Default|GetDFDisk))
  (bind (_origin _boxextent _sphereradius) (Collision|GetComponentBounds _dfdisk))
  (bind _returnvalue (Class|GameplayStatics|GrassOverlappingSphereCount (Variables|Default|GetGrassMesh) _origin _sphereradius))
  (return _returnvalue))

(fn UpdateMesh
  (if (Variables|Default|GetisTimerSet)
    _
    (else
      (Variables|Default|SetStartTime (Utilities|Time|GetGameTimeinSeconds))
      (Variables|Default|SetisTimerSet true)))
  (Transformation|SetWorldScale3D (Variables|Default|GetDFDisk) (Math|Vector|MakeVector (Math|Float|Lerp 0.0 (Variables|Default|GetFinalScaleXY) (/ (- (Utilities|Time|GetGameTimeinSeconds) (Variables|Default|GetStartTime)) (Variables|Default|GetAnimationTime))) (Math|Float|Lerp 0.0 (Variables|Default|GetFinalScaleXY) (/ (- (Utilities|Time|GetGameTimeinSeconds) (Variables|Default|GetStartTime)) (Variables|Default|GetAnimationTime))) 0.5))
  (if (>= (- (Utilities|Time|GetGameTimeinSeconds) (Variables|Default|GetStartTime)) (Variables|Default|GetAnimationTime))
    (Variables|Default|SetisTimerSet false)
    (Utilities|Time|ClearandInvalidateTimerbyHandle (Variables|Default|GetTimerHandle))))