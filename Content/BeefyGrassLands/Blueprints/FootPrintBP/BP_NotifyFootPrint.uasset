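; BP_NotifyFootPrint is an animation notify that triggers grass footprint effects during character animations.
; On notify, it looks for a BP_BeefyGrassComponent on the animated mesh's owner and acts only if that component is valid.
; It reads the world location of the FootSocketName socket and passes it to the component to spawn both vector field and grass footprint particles.
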(fn ReceivedNotify
  (params (MeshComp :type Skeletal%20Mesh%20Component%20Object%20Reference) (Animation :type Anim%20Sequence%20Base%20Object%20Reference))
  (bind _returnvalue (Components|GetOwner MeshComp))
  (bind _returnvalue_2 (Actor|GetComponentbyClass _returnvalue "/Game/BeefyGrassLands/Blueprints/Components/BP_BeefyGrassComponent.BP_BeefyGrassComponent_C"))
  (Utilities|IsValid _returnvalue_2
    (:Is%20Valid
      (LocalVariables|SetBeefyGrassComp _returnvalue_2)
      (LocalVariables|SetNewLocation (Transformation|GetSocketLocation MeshComp (Variables|Default|GetFootSocketName)))
      (Default|SpawnVectorFieldFootPrintParticle (LocalVariables|GetBeefyGrassComp) (LocalVariables|GetNewLocation))
      (Default|SpawnGrassFootPrintParticle (LocalVariables|GetBeefyGrassComp) (LocalVariables|GetNewLocation))
      (return false))))