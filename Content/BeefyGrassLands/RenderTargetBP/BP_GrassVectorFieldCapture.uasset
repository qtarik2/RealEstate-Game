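; Orthographic scene capture actor that follows the player to capture a vector field for grass, showing only a background component plus components registered through AddToSceneCaptureList.
; A looping timer moves it to the MPC_Level PlayerLocation plus a height offset, rather than using Tick.
; It writes CaptureLocation and CaptureSize back to MPC_Level so materials can locate the captured area.
; SnapToPixelWorldSize holds only unused pixel-snapping math, so movement is unsnapped.
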(event EventBeginPlay
  (Main|SetCaptureSize)
  (Main|MoveCapture)
  (Utilities|Time|SetTimerbyFunctionName 0 "MoveCapture" (Variables|Default|GetMoveUpdateInterval) true))

(event EventTick
  (params (DeltaSeconds :type Float%20%28single-precision%29)))

(fn ConstructionScript
  (Main|SetCaptureSize)
  (Main|MoveCapture)
  (Rendering|SceneCapture|ShowOnlyComponent (Variables|Default|GetSceneCaptureComponent2D) (Variables|Default|GetVectorFieldBackground)))

(fn MoveCapture
  (bind _returnvalue (Rendering|Material|GetVectorParameterValue "/Game/BeefyGrassLands/MPC_Level.MPC_Level" "PlayerLocation" :!class /Script/Engine.KismetMaterialLibrary))
  (Variables|Default|SetCaptureLocation (Math|Vector|MakeVector (.r _returnvalue) (.g _returnvalue) (+ (.b _returnvalue) (Variables|Default|GetRenderHeightOffset))))
  (Transformation|SetActorLocation (Variables|Default|GetCaptureLocation) false false)
  (Rendering|Material|SetVectorParameterValue "/Game/BeefyGrassLands/MPC_Level.MPC_Level" "CaptureLocation" (Math|Conversions|ToLinearColor(Vector) (Variables|Default|GetCaptureLocation)) :!class /Script/Engine.KismetMaterialLibrary))

(fn SetCaptureSize
  (Rendering|Material|SetScalarParameterValue "/Game/BeefyGrassLands/MPC_Level.MPC_Level" "CaptureSize" (Variables|Default|GetRenderOrthoWidth) :!class /Script/Engine.KismetMaterialLibrary)
  (Variables|/Script/Engine.SceneCaptureComponent2D|SetOrthoWidth (Variables|Default|GetSceneCaptureComponent2D) (Variables|Default|GetRenderOrthoWidth)))

(fn AddtoSceneCaptureList
  (params (Comp :type Primitive%20Component%20Object%20Reference))
  (Rendering|SceneCapture|ShowOnlyComponent (Variables|Default|GetSceneCaptureComponent2D) Comp))