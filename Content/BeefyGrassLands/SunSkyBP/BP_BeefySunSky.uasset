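; Sun and sky actor that sets sun position, light intensity and optional color temperature from a time of day.
; Construction calls inherited sun/sky updates, scales lighting by sun height and writes sun direction to MPC_Level for materials.
; SunSkyUpdate advances the clock and calendar from game time over a configurable day length.
; Its BeginPlay timer is disabled by a false branch, so the cycle does not start itself.
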(event EventBeginPlay
  (CallFunction|SaveSunDirection)
  (if false
    (bind _returnvalue (Utilities|Time|SetTimerbyFunctionName 0 "SunSkyUpdate" (Variables|Settings|GetUpdateInterval%20%28Seconds%29) true))
    (Variables|Default|SetTimerHandle _returnvalue)))

(fn ConstructionScript
  (|CallParentFunction)
  (bind _output_get (Variables|Default|SetOneDay (* 60 (Variables|Settings|GetDayLength%20%28Minutes%29))))
  (Variables|Default|SetOneHour (/ _output_get 24.0))
  ;[1 1 1] Save Starting Time Of Day
  (Variables|Default|SetSolarTime (+ (Math|Conversions|ToFloat(Integer) (Variables|Settings|GetHours)) (/ (Math|Conversions|ToFloat(Integer) (Variables|Settings|GetMinutes)) 6e+01) (/ (Math|Conversions|ToFloat(Integer) (Variables|Settings|GetSeconds)) 3.6e+03)))
  (CallFunction|SaveSunDirection)
  (CallFunction|UpdateSun)
  (CallFunction|UpdateSky)
  (CallFunction|SetDayLightIntensity)
  (if (Variables|Settings|GetTemperatureAdjustment)
    (CallFunction|SetSunTemperature)))

(fn SaveSunDirection
  (Rendering|Material|SetVectorParameterValue "/Game/BeefyGrassLands/MPC_Level.MPC_Level" "Sun Direction" (Math|Conversions|ToLinearColor(Vector) (* (Math|Vector|GetForwardVector (Variables|Default|GetDirectionalLight)) -1.0)) :!class /Script/Engine.KismetMaterialLibrary))

(fn SetDayLightIntensity
  (bind _directionallight (Variables|Default|GetDirectionalLight))
  (bind _returnvalue (Math|Vector|GetForwardVector _directionallight))
  (bind _returnvalue_2 (* _returnvalue -1))
  (bind _z (Math|Vector|BreakVector _returnvalue_2))
  (Rendering|Components|Light|SetIntensity (Variables|Default|GetDirectionalLight) (* (Math|Float|Clamp(Float) (/ _z 0.1) 0.001) (Variables|Settings|GetSunLightIntensity)))
  (Rendering|Components|Light|SetIntensity (Variables|Default|GetSkyLight) (* (Math|Float|Clamp(Float) (/ (Math|Float|Clamp(Float) _z) (Variables|Default|GetLightBlendTransition)) 0.001) (Variables|Settings|GetSkyLightIntensity))))

(fn SetSunTemperature
  (bind _lightblendtransition (Variables|Default|GetLightBlendTransition))
  (bind _directionallight (Variables|Default|GetDirectionalLight))
  (bind _returnvalue (Math|Vector|GetForwardVector _directionallight))
  (bind _returnvalue_2 (* _returnvalue -1))
  (bind _z (Math|Vector|BreakVector _returnvalue_2))
  (bind _returnvalue_3 (Math|Float|Clamp(Float) _z))
  (bind _returnvalue_4 (/ _returnvalue_3 _lightblendtransition))
  (bind _returnvalue_5 (Math|Float|Clamp(Float) _returnvalue_4))
  (Class|LightComponent|SetTemperature (Variables|Default|GetDirectionalLight) (+ (* _returnvalue_5 (Variables|Settings|GetSun%20Temperature%20Offset)) (+ (* _returnvalue_5 3.5e+03) 2e+03))))

(fn SunSkyUpdate
  (bind _returnvalue (Utilities|Time|GetGameTimeinSeconds))
  ;[1 1 1] Increment Time
  (if (>= (+ (Variables|Default|GetSolarTime) (/ (- _returnvalue (Variables|Default|GetTimeElapsed)) (Variables|Default|GetOneHour))) 24.0)
    (Variables|Default|SetSolarTime 0.0)
    (Variables|Default|SetTimeElapsed _returnvalue)
    (if (Math|Boolean|ORBoolean false (and (== (+ (Variables|Default|GetDay) (Variables|Default|GetDayIncrements)) 31) (Math|Boolean|ORBoolean (>= (Variables|Default|GetMonth) 4) (>= (Variables|Default|GetMonth) 6) (>= (Variables|Default|GetMonth) 9) (>= (Variables|Default|GetMonth) 11))) (>= (+ (Variables|Default|GetDay) (Variables|Default|GetDayIncrements)) 32))
      (Variables|Default|SetDay 1)
      (if (== (+ (Variables|Default|GetMonth) (Variables|Default|GetMonthIncrement)) 13)
        (Variables|Default|SetMonth 1)
        (else
          (Variables|Default|SetMonth (+ (Variables|Default|GetMonth) (Variables|Default|GetMonthIncrement)))))
      (else
        (Variables|Default|SetDay (+ (Variables|Default|GetDay) (Variables|Default|GetDayIncrements)))))
    (else
      (Variables|Default|SetSolarTime (+ (Variables|Default|GetSolarTime) (/ (- _returnvalue (Variables|Default|GetTimeElapsed)) (Variables|Default|GetOneHour))))
      (Variables|Default|SetTimeElapsed _returnvalue)))
  ;[1 1 1] Update SunPos Variables
  (Variables|Settings|SetHours (Math|Float|Truncate (Variables|Default|GetSolarTime)))
  (Variables|Settings|SetMinutes (Math|Float|Truncate (* (Math|Float|Fraction (Variables|Default|GetSolarTime)) 6e+01)))
  (Variables|Settings|SetSeconds (Math|Float|Truncate (* (Math|Float|Fraction (* (Math|Float|Fraction (Variables|Default|GetSolarTime)) 6e+01)) 6e+01)))
  (CallFunction|UpdateSun)
  (if (Variables|Settings|GetTemperatureAdjustment)
    (CallFunction|SetDayLightIntensity))
  (CallFunction|SetSunTemperature))