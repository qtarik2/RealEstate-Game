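; Sun positioner actor that runs a day/night cycle with calendar rollover, driving the sky sphere's directional light and a sky light.
; A looping timer, when enabled, advances time from a configurable day length and calls UpdateSun.
; Sun elevation then sets color temperature and optionally both light intensities, while sun direction is written to MPC_Level for materials.
; Construction finds a missing sky light, applies initial lighting and recaptures the sky.
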(event EventBeginPlay
  (CallFunction|SaveSunDirection)
  (if (Variables|Default|GetTimer%20Update)
    (bind _returnvalue (Utilities|Time|SetTimerbyFunctionName 0 "SunPositionUpdate" (Variables|Default|GetUpdateInterval%20%28Seconds%29) true))
    (Variables|Default|SetTimerHandle _returnvalue)))

(fn ConstructionScript
  (|CallParentFunction)
  (bind _output_get (Variables|Default|SetOneDay (* 60 (Variables|Default|GetDayLength%20%28Minutes%29))))
  (Variables|Default|SetOneHour (/ _output_get 24.0))
  ;[1 1 1] If no sky light actor is set, find one and assign it
  (if (Utilities|IsValidSoftObjectReference (Utilities|ResolveSoftReference (Variables|Default|GetSky%20Light)))
    (if (Variables|Default|GetTimer%20Update) :!label _label
      (Transformation|SetMobility (Variables|/Script/Engine.Light|GetLightComponent (Variables|/Engine/EngineSky/BP_Sky_Sphere.BP_Sky_Sphere_C|GetDirectional%20light%20actor (Utilities|ResolveSoftReference (Variables|Default|GetSkySphere)))) "Movable"))
    ;[1 1 1] Save Starting Time Of Day
    (Variables|Default|SetTimeOfDay (+ (Math|Conversions|ToFloat(Integer) (Variables|Default|GetHours)) (/ (Math|Conversions|ToFloat(Integer) (Variables|Default|GetMinutes)) 6e+01) (/ (Math|Conversions|ToFloat(Integer) (Variables|Default|GetSeconds)) 3.6e+03)))
    (CallFunction|SaveSunDirection)
    (CallFunction|SetDayLightIntensity)
    (CallFunction|SetSunTemperature)
    (Class|SkyLightComponent|RecaptureSky (Variables|/Script/Engine.SkyLight|GetLightComponent (Variables|Default|GetSky%20Light)))
    (else
      (bind _outactors (Actor|GetAllActorsOfClass "/Script/Engine.SkyLight"))
      (if (> (Utilities|Array|Length _outactors) 0)
        (Variables|Default|SetSky%20Light (Utilities|Array|Get(acopy) _outactors))
        (goto _label)))))

(fn SetSunTemperature
  (bind _daylight_transition (Variables|Default|GetDaylight%20Transition))
  (bind _skysphere (Variables|Default|GetSkySphere))
  (bind _output (Utilities|ResolveSoftReference _skysphere))
  (bind _directional_light_actor (Variables|/Engine/EngineSky/BP_Sky_Sphere.BP_Sky_Sphere_C|GetDirectional%20light%20actor _output))
  (bind _rootcomponent (Variables|/Script/Engine.Actor|GetRootComponent _directional_light_actor))
  (bind _returnvalue (Math|Vector|GetForwardVector _rootcomponent))
  (bind _returnvalue_2 (* _returnvalue -1))
  (bind _z (Math|Vector|BreakVector _returnvalue_2))
  (bind _returnvalue_3 (Math|Float|Clamp(Float) _z))
  (bind _returnvalue_4 (/ _returnvalue_3 _daylight_transition))
  (bind _returnvalue_5 (Math|Float|Clamp(Float) _returnvalue_4))
  ;[1 1 1] Set Sun Temperature
  (Class|LightComponent|SetTemperature (Variables|/Script/Engine.Light|GetLightComponent (Variables|/Engine/EngineSky/BP_Sky_Sphere.BP_Sky_Sphere_C|GetDirectional%20light%20actor (Utilities|ResolveSoftReference (Variables|Default|GetSkySphere)))) (+ (* _returnvalue_5 (Variables|Default|GetSun%20Temperature%20Offset)) (+ (* _returnvalue_5 3.5e+03) 2e+03))))

(fn SaveSunDirection
  ;[1 1 1] Sun Direction Param.
  (Rendering|Material|SetVectorParameterValue "/Game/BeefyGrassLands/MPC_Level.MPC_Level" "Sun Direction" (Math|Conversions|ToLinearColor(Vector) (* (Math|Vector|GetForwardVector (Variables|/Script/Engine.Actor|GetRootComponent (Variables|/Engine/EngineSky/BP_Sky_Sphere.BP_Sky_Sphere_C|GetDirectional%20light%20actor (Utilities|ResolveSoftReference (Variables|Default|GetSkySphere))))) -1)) :!class /Script/Engine.KismetMaterialLibrary))

(fn SetDayLightIntensity
  (bind _skysphere (Variables|Default|GetSkySphere))
  (bind _output (Utilities|ResolveSoftReference _skysphere))
  (bind _directional_light_actor (Variables|/Engine/EngineSky/BP_Sky_Sphere.BP_Sky_Sphere_C|GetDirectional%20light%20actor _output))
  (bind _rootcomponent (Variables|/Script/Engine.Actor|GetRootComponent _directional_light_actor))
  (bind _returnvalue (Math|Vector|GetForwardVector _rootcomponent))
  (bind _returnvalue_2 (* _returnvalue -1))
  (bind _z (Math|Vector|BreakVector _returnvalue_2))
  ;[1 1 1] Set Day / Night Intensity
  (Rendering|Components|Light|SetIntensity (Variables|/Script/Engine.Light|GetLightComponent (Variables|/Engine/EngineSky/BP_Sky_Sphere.BP_Sky_Sphere_C|GetDirectional%20light%20actor (Utilities|ResolveSoftReference (Variables|Default|GetSkySphere)))) (* (Math|Float|Clamp(Float) (/ _z 0.1) 0.001) (Variables|Default|GetSun%20Light%20Intensity)))
  (Rendering|Components|Light|SetIntensity (Variables|/Script/Engine.SkyLight|GetLightComponent (Variables|Default|GetSky%20Light)) (* (Math|Float|Clamp(Float) (/ (Math|Float|Clamp(Float) _z) (Variables|Default|GetDaylight%20Transition)) 0.001) (Variables|Default|GetSky%20Light%20Intensity))))

(fn SunPositionUpdate
  (bind _returnvalue (Utilities|Time|GetGameTimeinSeconds))
  ;[1 1 1] Increment Time
  (if (>= (+ (Variables|Default|GetTimeOfDay) (/ (- _returnvalue (Variables|Default|GetTimeElapsed)) (Variables|Default|GetOneHour))) 24.0)
    (Variables|Default|SetTimeOfDay 0.0)
    (Variables|Default|SetTimeElapsed _returnvalue)
    (if (Math|Boolean|ORBoolean (and (>= (+ (Variables|Default|GetDay) (Variables|Default|GetDayIncrements)) (+ (- 1 (Math|Integer|Clamp(Integer) (Math|Integer|%(Integer) (Variables|Default|GetYear) 4) 0 1)) 29)) (== (Variables|Default|GetMonth) 2)) (and (== (+ (Variables|Default|GetDay) (Variables|Default|GetDayIncrements)) 31) (Math|Boolean|ORBoolean (>= (Variables|Default|GetMonth) 4) (>= (Variables|Default|GetMonth) 6) (>= (Variables|Default|GetMonth) 9) (>= (Variables|Default|GetMonth) 11))) (>= (+ (Variables|Default|GetDay) (Variables|Default|GetDayIncrements)) 32))
      (Variables|Default|SetDay 1)
      (if (== (+ (Variables|Default|GetMonth) (Variables|Default|GetMonthIncrement)) 13)
        (Variables|Default|SetMonth 1)
        (if (== (+ (Variables|Default|GetYear) (Variables|Default|GetYearIncrement)) 2201)
          (Variables|Default|SetYear 1800)
          (else
            (Variables|Default|SetYear (+ (Variables|Default|GetYear) (Variables|Default|GetYearIncrement)))))
        (else
          (Variables|Default|SetMonth (+ (Variables|Default|GetMonth) (Variables|Default|GetMonthIncrement)))))
      (else
        (Variables|Default|SetDay (+ (Variables|Default|GetDay) (Variables|Default|GetDayIncrements)))))
    (else
      (Variables|Default|SetTimeOfDay (+ (Variables|Default|GetTimeOfDay) (/ (- _returnvalue (Variables|Default|GetTimeElapsed)) (Variables|Default|GetOneHour))))
      (Variables|Default|SetTimeElapsed _returnvalue)))
  ;[1 1 1] Update SunPos Variables
  (Variables|Default|SetHours (Math|Float|Truncate (Variables|Default|GetTimeOfDay)))
  (Variables|Default|SetMinutes (Math|Float|Truncate (* (Math|Float|Fraction (Variables|Default|GetTimeOfDay)) 6e+01)))
  (Variables|Default|SetSeconds (Math|Float|Truncate (* (Math|Float|Fraction (* (Math|Float|Fraction (Variables|Default|GetTimeOfDay)) 6e+01)) 6e+01)))
  (CallFunction|UpdateSun)
  (CallFunction|SaveSunDirection)
  (if (Variables|Default|GetLight%20Adjustments)
    (CallFunction|SetDayLightIntensity))
  (CallFunction|SetSunTemperature))