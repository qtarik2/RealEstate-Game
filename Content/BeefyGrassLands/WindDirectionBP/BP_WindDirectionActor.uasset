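; Wind controller actor that writes global, grass and stalk wind settings, with direction taken from its arrow, into the MPC_Level parameter collection.
; Settings apply on construction and BeginPlay; an optional looping timer alternates between max and alternate speeds.
; Each shift publishes acceleration, start time and accumulated displacement and location instead of ticking, then a timer finalizes the new speed.
; UpdateWindDirection can interpolate direction, but nothing here calls it.
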(event EventBeginPlay
  (Main|InitializeParameters)
  (if (Variables|Main|GetAlternatingWindSpeed)
    (Utilities|Time|SetTimerbyFunctionName 0 "AlternateWindSpeed" (Variables|Main|GetWindShiftInterval) true)))

(fn ConstructionScript
  (Main|InitializeParameters))

(fn InitializeParameters
  (Variables|Main|SetGlobalWindSpeed (Variables|Main|GetGlobalWindSpeedMax))
  (Variables|Main|SetWindDirection (Math|Vector|GetForwardVector (Variables|Default|GetWind%20Direction%20Arrow)))
  (Rendering|Material|SetVectorParameterValue "/Game/BeefyGrassLands/MPC_Level.MPC_Level" "WindDirection" (Math|Conversions|ToLinearColor(Vector) (Variables|Main|GetWindDirection)) :!class /Script/Engine.KismetMaterialLibrary)
  (Rendering|Material|SetScalarParameterValue "/Game/BeefyGrassLands/MPC_Level.MPC_Level" "GlobalWindSpeed" (Variables|Main|GetGlobalWindSpeed) :!class /Script/Engine.KismetMaterialLibrary)
  (Rendering|Material|SetScalarParameterValue "/Game/BeefyGrassLands/MPC_Level.MPC_Level" "GlobalWindAngle" (Variables|Main|GetGlobalWindAngle) :!class /Script/Engine.KismetMaterialLibrary)
  (Rendering|Material|SetScalarParameterValue "/Game/BeefyGrassLands/MPC_Level.MPC_Level" "GrassWindSpeed" (Variables|GrassSettings|GetGrassWindSpeed) :!class /Script/Engine.KismetMaterialLibrary)
  (Rendering|Material|SetScalarParameterValue "/Game/BeefyGrassLands/MPC_Level.MPC_Level" "GrassWindRotation" (Variables|GrassSettings|GetGrassWindAngle) :!class /Script/Engine.KismetMaterialLibrary)
  (Rendering|Material|SetScalarParameterValue "/Game/BeefyGrassLands/MPC_Level.MPC_Level" "GrassWindGustScale" (Variables|GrassSettings|GetGrassWindGustScale) :!class /Script/Engine.KismetMaterialLibrary)
  (Rendering|Material|SetScalarParameterValue "/Game/BeefyGrassLands/MPC_Level.MPC_Level" "GrassWindGustSpeed" (Variables|GrassSettings|GetGrassWindGustSpeed) :!class /Script/Engine.KismetMaterialLibrary)
  (Rendering|Material|SetScalarParameterValue "/Game/BeefyGrassLands/MPC_Level.MPC_Level" "GrassWindResistance" (Variables|GrassSettings|GetGrassWindResistance) :!class /Script/Engine.KismetMaterialLibrary)
  (Rendering|Material|SetScalarParameterValue "/Game/BeefyGrassLands/MPC_Level.MPC_Level" "GrassWindOffsetAngle" (Variables|GrassSettings|GetGrassWindOffset) :!class /Script/Engine.KismetMaterialLibrary)
  (Rendering|Material|SetScalarParameterValue "/Game/BeefyGrassLands/MPC_Level.MPC_Level" "GrassWindShelterBias" (Variables|GrassSettings|GetGrassWindShelterBias) :!class /Script/Engine.KismetMaterialLibrary)
  (Rendering|Material|SetScalarParameterValue "/Game/BeefyGrassLands/MPC_Level.MPC_Level" "GrassWindShelterModulation" (Variables|GrassSettings|GetGrassWindShelterModulation) :!class /Script/Engine.KismetMaterialLibrary)
  (Rendering|Material|SetScalarParameterValue "/Game/BeefyGrassLands/MPC_Level.MPC_Level" "GrassRandomWindChange" (Variables|GrassSettings|GetGrassRandomWindChange) :!class /Script/Engine.KismetMaterialLibrary)
  (Rendering|Material|SetScalarParameterValue "/Game/BeefyGrassLands/MPC_Level.MPC_Level" "GrassRandomWindInfluence" (Variables|GrassSettings|GetGrassRandomWindInfluence) :!class /Script/Engine.KismetMaterialLibrary)
  (Rendering|Material|SetScalarParameterValue "/Game/BeefyGrassLands/MPC_Level.MPC_Level" "StalkWindResistance" (Variables|GrassSettings|GetStalkWindResistance) :!class /Script/Engine.KismetMaterialLibrary)
  (Rendering|Material|SetScalarParameterValue "/Game/BeefyGrassLands/MPC_Level.MPC_Level" "StalkWindOffsetAngle" (Variables|GrassSettings|GetStalkWindOffset) :!class /Script/Engine.KismetMaterialLibrary))

(fn StartWindShift
  (params (NewDirection :type Vector :default "1.000000,0,0") (NewIntensity :type Float%20%28single-precision%29))
  (if (not (Variables|Main|GetIsTimerSet))
    (Variables|Main|SetIsTimerSet true)
    (Variables|WindShift|SetNewWindDirection NewDirection)
    (Variables|WindShift|SetStartWindDirection (Variables|Main|GetWindDirection))
    (Variables|WindShift|SetNewWindSpeed NewIntensity)
    (bind _output_get (Variables|WindShift|SetWindDisplacement (+ (* (- (Utilities|Time|GetGameTimeinSeconds) (Variables|WindShift|GetStartTime)) (Variables|Main|GetGlobalWindSpeed)) (Variables|WindShift|GetWindDisplacement))))
    (Rendering|Material|SetScalarParameterValue "/Game/BeefyGrassLands/MPC_Level.MPC_Level" "WindDisplacement" _output_get :!class /Script/Engine.KismetMaterialLibrary)
    (bind _output_get_2 (Variables|WindShift|SetWindLocationOffset (+ (* (Variables|Main|GetWindDirection) (* (- (Utilities|Time|GetGameTimeinSeconds) (Variables|WindShift|GetStartTime)) (Variables|Main|GetGlobalWindSpeed))) (Variables|WindShift|GetWindLocationOffset))))
    (Rendering|Material|SetVectorParameterValue "/Game/BeefyGrassLands/MPC_Level.MPC_Level" "WindLocation" (Math|Conversions|ToLinearColor(Vector) _output_get_2) :!class /Script/Engine.KismetMaterialLibrary)
    (bind _output_get_3 (Variables|WindShift|SetWindAcceleration (/ (- NewIntensity (Variables|Main|GetGlobalWindSpeed)) (Variables|Main|GetWindShiftDuration))))
    (Rendering|Material|SetScalarParameterValue "/Game/BeefyGrassLands/MPC_Level.MPC_Level" "WindAcceleration" _output_get_3 :!class /Script/Engine.KismetMaterialLibrary)
    (bind _output_get_4 (Variables|WindShift|SetStartTime (Utilities|Time|GetGameTimeinSeconds)))
    (Rendering|Material|SetScalarParameterValue "/Game/BeefyGrassLands/MPC_Level.MPC_Level" "WindStartTime" _output_get_4 :!class /Script/Engine.KismetMaterialLibrary)
    (bind _returnvalue (Utilities|Time|SetTimerbyFunctionName 0 "EndWindShift" (Variables|Main|GetWindShiftDuration)))
    (Variables|Main|SetUpdateTimerHandle _returnvalue)))

(fn EndWindShift
  (bind _output_get (Variables|WindShift|SetWindDisplacement (+ (Utilities|GetWindDisplacement (Variables|Main|GetWindShiftDuration)) (Variables|WindShift|GetWindDisplacement))))
  (Rendering|Material|SetScalarParameterValue "/Game/BeefyGrassLands/MPC_Level.MPC_Level" "WindDisplacement" _output_get :!class /Script/Engine.KismetMaterialLibrary)
  (bind _output_get_2 (Variables|WindShift|SetWindLocationOffset (+ (* (Variables|Main|GetWindDirection) (Utilities|GetWindDisplacement (Variables|Main|GetWindShiftDuration))) (Variables|WindShift|GetWindLocationOffset))))
  (Rendering|Material|SetVectorParameterValue "/Game/BeefyGrassLands/MPC_Level.MPC_Level" "WindLocation" (Math|Conversions|ToLinearColor(Vector) _output_get_2) :!class /Script/Engine.KismetMaterialLibrary)
  (bind _output_get_3 (Variables|WindShift|SetWindAcceleration 0.0))
  (Rendering|Material|SetScalarParameterValue "/Game/BeefyGrassLands/MPC_Level.MPC_Level" "WindAcceleration" _output_get_3 :!class /Script/Engine.KismetMaterialLibrary)
  (bind _output_get_4 (Variables|Main|SetGlobalWindSpeed (Variables|WindShift|GetNewWindSpeed)))
  (Rendering|Material|SetScalarParameterValue "/Game/BeefyGrassLands/MPC_Level.MPC_Level" "GlobalWindSpeed" _output_get_4 :!class /Script/Engine.KismetMaterialLibrary)
  (bind _output_get_5 (Variables|WindShift|SetStartTime (Utilities|Time|GetGameTimeinSeconds)))
  (Rendering|Material|SetScalarParameterValue "/Game/BeefyGrassLands/MPC_Level.MPC_Level" "WindStartTime" _output_get_5 :!class /Script/Engine.KismetMaterialLibrary)
  (Variables|Main|SetIsTimerSet false))

(fn UpdateWindDirection
  (LocalVariables|SetDeltaTime (- (Utilities|Time|GetGameTimeinSeconds) (Variables|WindShift|GetStartTime)))
  (bind _output_get (Variables|Main|SetWindDirection (Math|Vector|GetForwardVector (Math|Rotator|Lerp(Rotator) (Math|Conversions|RotationFromXVector (Variables|WindShift|GetStartWindDirection)) (Math|Conversions|RotationFromXVector (Variables|WindShift|GetNewWindDirection)) (/ (LocalVariables|GetDeltaTime) (Variables|Main|GetWindShiftDuration))))))
  (Rendering|Material|SetVectorParameterValue "/Game/BeefyGrassLands/MPC_Level.MPC_Level" "WindDirection" (Math|Conversions|ToLinearColor(Vector) _output_get) :!class /Script/Engine.KismetMaterialLibrary)
  (if (>= (LocalVariables|GetDeltaTime) (Variables|Main|GetWindShiftDuration))
    (Utilities|Time|ClearandInvalidateTimerbyHandle (Variables|Main|GetUpdateTimerHandle))
    (Variables|Main|SetIsTimerSet false)))

(fn AlternateWindSpeed
  (bind _globalwindspeed__alt_ (Variables|Main|GetGlobalWindSpeed%20%28Alt%29))
  (Variables|Main|SetWindSwitch (- 1.0 (Variables|Main|GetWindSwitch)))
  (Main|StartWindShift (Variables|Main|GetWindDirection) (+ (* (Variables|Main|GetWindSwitch) (- (Variables|Main|GetGlobalWindSpeedMax) _globalwindspeed__alt_)) _globalwindspeed__alt_)))