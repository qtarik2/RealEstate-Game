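; BP_Brocoli is a broccoli crop actor that grows on spawn and harvests itself automatically after a fixed delay.
; BeginPlay starts the Growth timeline, whose PlantSize track sets the world scale of the many plant meshes.
; After the delay, LooseBrocoli destroys those meshes, spawns BrocoliLoose at LooseSpawn and plays a harvest sound, then the Widget is hidden.
; The timeline's Update also runs its own Delay before stopping Growth.
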(event Custom|GrowBrocoli
  (bind _plant_size (Timeline|Growth Play)
    (:Update
      (Transformation|SetWorldScale3D (Variables|Default|GetStaticMesh11) (Math|Conversions|ToVector(Float) _plant_size))
      (Utilities|FlowControl|Delay 5.0)
      (Timeline|Growth Stop))))

(event EventBeginPlay
  (CallFunction|GrowBrocoli)
  (Utilities|FlowControl|Delay 5.0)
  (CallFunction|LooseBrocoli)
  (Rendering|SetVisibility (Variables|Default|GetWidget) false false))

(fn ConstructionScript)

(fn LooseBrocoli
  (Components|DestroyComponent (Variables|Default|GetStaticMesh13))
  (Game|SpawnActorfromClass "/Game/ActorsBP/CropLoose/ReadyCrops/BrocoliLoose.BrocoliLoose_C" (Transformation|GetWorldTransform (Variables|Default|GetLooseSpawn)) "Undefined" 0 0)
  (Audio|PlaySound2D "/Game/Sound_Effects/CropingAndHarvestingCropsSounds/HarvestingSound/Harvest_Crop_Activities_2.Harvest_Crop_Activities_2" 1.0 1.0 0.0 0 0))