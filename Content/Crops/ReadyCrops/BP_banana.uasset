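; Banana crop actor that animates the plant's growth, then swaps it for loose bananas.
; On BeginPlay the Growth timeline drives the world scale of the many plant meshes, with a delayed stop triggered from its update.
; After a fixed delay, LooseBanana destroys those meshes and the CropTile, spawns BP_BananaLoose at CropTile1 and plays a harvest sound, then the widget is hidden.
; The randomized grow-time nodes are unused.
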(event Custom|GrowBanana
  (bind _plant_size (Timeline|Growth Play)
    (:Update
      (Transformation|SetWorldScale3D (Variables|Default|GetStaticMesh109) (Math|Conversions|ToVector(Float) _plant_size))
      (Utilities|FlowControl|Delay 5.0)
      (Timeline|Growth Stop))))

(event EventBeginPlay
  (CallFunction|GrowBanana)
  (Utilities|FlowControl|Delay 5.0)
  (CallFunction|LooseBanana)
  (Rendering|SetVisibility (Variables|Default|GetWidget) false false))

(fn ConstructionScript)

(fn LooseBanana
  (Components|DestroyComponent (Variables|Default|GetStaticMesh96))
  (Game|SpawnActorfromClass "/Game/ActorsBP/CropLoose/ReadyCrops/BP_BananaLoose.BP_BananaLoose_C" (Transformation|GetWorldTransform (Variables|Default|GetCropTile1)) "Undefined" 0 0)
  (Audio|PlaySound2D "/Game/Sound_Effects/CropingAndHarvestingCropsSounds/HarvestingSound/Harvest_Crop_Activities_2.Harvest_Crop_Activities_2" 1.0 1.0 0.0 0 0))