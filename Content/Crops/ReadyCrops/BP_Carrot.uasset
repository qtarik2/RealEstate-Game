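; BP_Carrot is a carrot crop actor that grows a field of carrot meshes and then harvests itself automatically.
; On BeginPlay, the Growth timeline scales every carrot component together, stopping after a short delay.
; After a matching fixed delay, LooseCarrot destroys those meshes, spawns BP_CarrotLoose at LooseCarrotPoint and plays a harvest sound.
; The widget is then hidden, while the actor itself is not destroyed.
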(event Custom|GrowCarrot
  (bind _plant_size (Timeline|Growth Play)
    (:Update
      (Transformation|SetWorldScale3D (Variables|Default|GetCarrot12) (Math|Conversions|ToVector(Float) _plant_size))
      (Utilities|FlowControl|Delay 5.0)
      (Timeline|Growth Stop))))

(event EventBeginPlay
  (CallFunction|GrowCarrot)
  (Utilities|FlowControl|Delay 5.0)
  (CallFunction|LooseCarrot)
  (Rendering|SetVisibility (Variables|Default|GetWidget) false false))

(fn ConstructionScript)

(fn LooseCarrot
  (Components|DestroyComponent (Variables|Default|GetCarrot122))
  (Game|SpawnActorfromClass "/Game/ActorsBP/CropLoose/ReadyCrops/BP_CarrotLoose.BP_CarrotLoose_C" (Transformation|GetWorldTransform (Variables|Default|GetLooseCarrot%20Point)) "Undefined" 0 0)
  (Audio|PlaySound2D "/Game/Sound_Effects/CropingAndHarvestingCropsSounds/HarvestingSound/Harvest_Crop_Activities_2.Harvest_Crop_Activities_2" 1.0 1.0 0.0 0 0))