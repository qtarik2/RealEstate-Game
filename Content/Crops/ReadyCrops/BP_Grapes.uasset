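; BP_Grapes is a grape crop actor that grows on spawn, then gives way to loose grapes.
; On BeginPlay, a Growth timeline scales the plant's static meshes, with a delayed Stop triggered from its update.
; After a random delay bounded by the two grow-time variables, it destroys the plant meshes, including EggPlantBase, and spawns a LooseGrapes actor at a remaining mesh's transform.
; It then hides its widget.
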(event Custom|GrowGrapes
  (bind _plant_size (Timeline|Growth Play)
    (:Update
      (Transformation|SetWorldScale3D (Variables|Default|GetStaticMesh55) (Math|Conversions|ToVector(Float) _plant_size))
      (Utilities|FlowControl|Delay (Variables|Default|GetGrapesGrowTime))
      (Timeline|Growth Stop))))

(event EventBeginPlay
  (CallFunction|GrowGrapes)
  (Utilities|FlowControl|Delay (Math|Random|RandomFloatinRange (Variables|Default|GetGrapesGrowTime) (Variables|Default|GetGrapesNewGrowTime)))
  (CallFunction|LooseGrapes)
  (Rendering|SetVisibility (Variables|Default|GetWidget) false false))

(fn ConstructionScript)

(fn LooseGrapes
  (Components|DestroyComponent (Variables|Default|GetStaticMesh62))
  (Game|SpawnActorfromClass "/Game/ActorsBP/CropLoose/ReadyCrops/looseGrapes.looseGrapes_C" (Transformation|GetWorldTransform (Variables|Default|GetStaticMesh70)) "Undefined" 0 0))