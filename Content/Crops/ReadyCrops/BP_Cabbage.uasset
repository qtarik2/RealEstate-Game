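; Cabbage crop actor that grows automatically on BeginPlay and turns into harvested loose cabbage after a fixed delay.
; The Growth timeline scales dozens of plant meshes together, with a delay in its update stopping the timeline.
; LooseCabbage then destroys those meshes and the crop tile and spawns BP_CabbageLoose at StaticMesh48's transform.
; Harvest and crunch sounds play, and the widget is hidden.
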(event Custom|GrowCabbage
  (bind _plant_size (Timeline|Growth Play)
    (:Update
      (Transformation|SetWorldScale3D (Variables|Default|GetStaticMesh11) (Math|Conversions|ToVector(Float) _plant_size))
      (Utilities|FlowControl|Delay 5.0)
      (Timeline|Growth Stop))))

(event EventBeginPlay
  (CallFunction|GrowCabbage)
  (Utilities|FlowControl|Delay 5.0)
  (CallFunction|LooseCabbage)
  (Audio|PlaySound2D "/Game/Sound_Effects/CropingAndHarvestingCropsSounds/Planting_Seeds/Crunch_of_a_Soft_Shell_3.Crunch_of_a_Soft_Shell_3" 1.0 1.0 0.0 0 0)
  (Rendering|SetVisibility (Variables|Default|GetWidget) false false))

(fn ConstructionScript)

(fn LooseCabbage
  (Components|DestroyComponent (Variables|Default|GetStaticMesh13))
  (Game|SpawnActorfromClass "/Game/ActorsBP/CropLoose/ReadyCrops/BP_CabbageLoose.BP_CabbageLoose_C" (Transformation|GetWorldTransform (Variables|Default|GetStaticMesh48)) "AdjustIfPossibleButDontSpawnIfColliding" 0 0)
  (Audio|PlaySound2D "/Game/Sound_Effects/CropingAndHarvestingCropsSounds/HarvestingSound/Harvest_Crop_Activities_2.Harvest_Crop_Activities_2" 1.0 1.0 0.0 0 0))