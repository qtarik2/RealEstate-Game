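; BP_pumpkin is a pumpkin crop that grows on BeginPlay, then becomes a loose pumpkin.
; A Growth timeline scales the plant's static meshes by its PlantSize track, with a delayed stop after PumpkinGrowTime.
; After a random delay between the two grow-time variables, PumpkinLoose destroys the plant meshes and spawns BP_PumpkinLoose at the LoosePumpkin component's transform.
; The widget is then hidden.
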(event Custom|GrowPumpkin
  (bind _plant_size (Timeline|Growth Play)
    (:Update
      (Transformation|SetWorldScale3D (Variables|Default|GetStaticMesh6) (Math|Conversions|ToVector(Float) _plant_size))
      (Utilities|FlowControl|Delay (Variables|Default|GetPumpkinGrowTime))
      (Timeline|Growth Stop))))

(event EventBeginPlay
  (CallFunction|GrowPumpkin)
  (Utilities|FlowControl|Delay (Math|Random|RandomFloatinRange (Variables|Default|GetPumpkinGrowTime) (Variables|Default|GetPumpkinNewGrowTime)))
  (CallFunction|PumpkinLoose)
  (Rendering|SetVisibility (Variables|Default|GetWidget) false false))

(fn ConstructionScript)

(fn PumpkinLoose
  (Components|DestroyComponent (Variables|Default|GetStaticMesh25))
  (Game|SpawnActorfromClass "/Game/ActorsBP/CropLoose/ReadyCrops/BP_PumpkinLoose.BP_PumpkinLoose_C" (Transformation|GetWorldTransform (Variables|Default|GetLoosePumpkin)) "Undefined" 0 0))