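; Cucumber crop actor that grows on BeginPlay, then turns into a loose cucumber.
; The Growth timeline drives the world scale of many static mesh components through its PlantSize track, with a five-second delay in its update that stops it.
; After a parallel five-second delay, LooseCucumber destroys the plant meshes and base, spawns a CucumberLoose actor at StaticMesh108's transform, and the widget is hidden.
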(event Custom|GrowCucumber
  (bind _plant_size (Timeline|Growth Play)
    (:Update
      (Transformation|SetWorldScale3D (Variables|Default|GetStaticMesh36) (Math|Conversions|ToVector(Float) _plant_size))
      (Utilities|FlowControl|Delay 5.0)
      (Timeline|Growth Stop))))

(event EventBeginPlay
  (CallFunction|GrowCucumber)
  (Utilities|FlowControl|Delay 5.0)
  (CallFunction|LooseCucumber)
  (Rendering|SetVisibility (Variables|Default|GetWidget) false false))

(fn ConstructionScript)

(fn LooseCucumber
  (Components|DestroyComponent (Variables|Default|GetStaticMesh66))
  (Game|SpawnActorfromClass "/Game/ActorsBP/CropLoose/ReadyCrops/CucumberLoose.CucumberLoose_C" (Transformation|GetWorldTransform (Variables|Default|GetStaticMesh108)) "Undefined" 0 0))