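; Hay crop actor that grows a field of plant meshes, then turns it into loose hay.
; On BeginPlay, the Growth timeline scales the meshes, with a delayed stop fired from its update.
; After a fixed delay, LooseHay destroys those meshes, spawns a LooseHay actor at one mesh's transform, and the widget is hidden.
; Per-component hover events switch the mouse cursor, mostly to crosshairs and back.
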(event OnBeginCursorOver(Wheat)
  (params (TouchedComponent :type Primitive%20Component%20Object%20Reference))
  (Variables|/Script/Engine.PlayerController|SetCurrentMouseCursor (Game|GetPlayerController 0) "Crosshairs"))

(event OnEndCursorOver(Wheat)
  (params (TouchedComponent :type Primitive%20Component%20Object%20Reference))
  (Variables|/Script/Engine.PlayerController|SetCurrentMouseCursor (Game|GetPlayerController 0) "Default"))

(event OnBeginCursorOver(StaticMesh20)
  (params (TouchedComponent :type Primitive%20Component%20Object%20Reference))
  (Variables|/Script/Engine.PlayerController|SetCurrentMouseCursor (Game|GetPlayerController 0) "Crosshairs"))

(event OnBeginCursorOver(StaticMesh25)
  (params (TouchedComponent :type Primitive%20Component%20Object%20Reference))
  (Variables|/Script/Engine.PlayerController|SetCurrentMouseCursor (Game|GetPlayerController 0) "Default"))

(event OnEndCursorOver(StaticMesh25)
  (params (TouchedComponent :type Primitive%20Component%20Object%20Reference))
  (Variables|/Script/Engine.PlayerController|SetCurrentMouseCursor (Game|GetPlayerController 0) "Default"))

(event OnEndCursorOver(StaticMesh23)
  (params (TouchedComponent :type Primitive%20Component%20Object%20Reference))
  (Variables|/Script/Engine.PlayerController|SetCurrentMouseCursor (Game|GetPlayerController 0) "Default"))

(event OnEndCursorOver(StaticMesh12)
  (params (TouchedComponent :type Primitive%20Component%20Object%20Reference))
  (Variables|/Script/Engine.PlayerController|SetCurrentMouseCursor (Game|GetPlayerController 0) "Default"))

(event OnEndCursorOver(StaticMesh2)
  (params (TouchedComponent :type Primitive%20Component%20Object%20Reference))
  (Variables|/Script/Engine.PlayerController|SetCurrentMouseCursor (Game|GetPlayerController 0) "Default"))

(event OnEndCursorOver(StaticMesh4)
  (params (TouchedComponent :type Primitive%20Component%20Object%20Reference))
  (Variables|/Script/Engine.PlayerController|SetCurrentMouseCursor (Game|GetPlayerController 0) "Default"))

(event OnEndCursorOver(StaticMesh11)
  (params (TouchedComponent :type Primitive%20Component%20Object%20Reference))
  (Variables|/Script/Engine.PlayerController|SetCurrentMouseCursor (Game|GetPlayerController 0) "Default"))

(event OnEndCursorOver(StaticMesh)
  (params (TouchedComponent :type Primitive%20Component%20Object%20Reference))
  (Variables|/Script/Engine.PlayerController|SetCurrentMouseCursor (Game|GetPlayerController 0) "Default"))

(event OnEndCursorOver(StaticMesh14)
  (params (TouchedComponent :type Primitive%20Component%20Object%20Reference))
  (Variables|/Script/Engine.PlayerController|SetCurrentMouseCursor (Game|GetPlayerController 0) "Default"))

(event OnBeginCursorOver(StaticMesh23)
  (params (TouchedComponent :type Primitive%20Component%20Object%20Reference))
  (Variables|/Script/Engine.PlayerController|SetCurrentMouseCursor (Game|GetPlayerController 0) "Crosshairs"))

(event OnEndCursorOver(StaticMesh18)
  (params (TouchedComponent :type Primitive%20Component%20Object%20Reference))
  (Variables|/Script/Engine.PlayerController|SetCurrentMouseCursor (Game|GetPlayerController 0) "Default"))

(event OnEndCursorOver(StaticMesh20)
  (params (TouchedComponent :type Primitive%20Component%20Object%20Reference))
  (Variables|/Script/Engine.PlayerController|SetCurrentMouseCursor (Game|GetPlayerController 0) "Default"))

(event OnBeginCursorOver(StaticMesh12)
  (params (TouchedComponent :type Primitive%20Component%20Object%20Reference))
  (Variables|/Script/Engine.PlayerController|SetCurrentMouseCursor (Game|GetPlayerController 0) "Crosshairs"))

(event OnBeginCursorOver(StaticMesh2)
  (params (TouchedComponent :type Primitive%20Component%20Object%20Reference))
  (Variables|/Script/Engine.PlayerController|SetCurrentMouseCursor (Game|GetPlayerController 0) "Crosshairs"))

(event OnBeginCursorOver(StaticMesh4)
  (params (TouchedComponent :type Primitive%20Component%20Object%20Reference))
  (Variables|/Script/Engine.PlayerController|SetCurrentMouseCursor (Game|GetPlayerController 0) "Crosshairs"))

(event OnBeginCursorOver(StaticMesh11)
  (params (TouchedComponent :type Primitive%20Component%20Object%20Reference))
  (Variables|/Script/Engine.PlayerController|SetCurrentMouseCursor (Game|GetPlayerController 0) "Crosshairs"))

(event OnBeginCursorOver(StaticMesh)
  (params (TouchedComponent :type Primitive%20Component%20Object%20Reference))
  (Variables|/Script/Engine.PlayerController|SetCurrentMouseCursor (Game|GetPlayerController 0) "Crosshairs"))

(event OnBeginCursorOver(StaticMesh14)
  (params (TouchedComponent :type Primitive%20Component%20Object%20Reference))
  (Variables|/Script/Engine.PlayerController|SetCurrentMouseCursor (Game|GetPlayerController 0) "Crosshairs"))

(event OnBeginCursorOver(StaticMesh18)
  (params (TouchedComponent :type Primitive%20Component%20Object%20Reference))
  (Variables|/Script/Engine.PlayerController|SetCurrentMouseCursor (Game|GetPlayerController 0) "Crosshairs"))

(event Custom|GrowCarrot
  (bind _plant_size (Timeline|Growth Play)
    (:Update
      (Transformation|SetWorldScale3D (Variables|Default|GetStaticMesh24) (Math|Conversions|ToVector(Float) _plant_size))
      (Utilities|FlowControl|Delay 5.0)
      (Timeline|Growth Stop))))

(event EventBeginPlay
  (CallFunction|GrowCarrot)
  (Utilities|FlowControl|Delay 1e+01)
  (CallFunction|LooseHay)
  (Rendering|SetVisibility (Variables|Default|GetWidget) false false))

(fn ConstructionScript)

(fn LooseHay
  (Components|DestroyComponent (Variables|Default|GetStaticMesh9))
  (Game|SpawnActorfromClass "/Game/ActorsBP/CropLoose/looseHay.looseHay_C" (Transformation|GetWorldTransform (Variables|Default|GetStaticMesh35)) "Undefined" 0 0))

(fn NewFunction0
  (Components|DestroyComponent (Variables|Default|GetStaticMesh14))
  (Game|SpawnActorfromClass "/Game/ActorsBP/CropLoose/looseHay.looseHay_C" (Transformation|GetWorldTransform (Variables|Default|GetStaticMesh35)) "Undefined" 0 0))