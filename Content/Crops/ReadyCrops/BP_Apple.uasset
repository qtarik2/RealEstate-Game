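; Apple crop actor that grows on spawn and automatically turns into loose apples after a fixed delay.
; BeginPlay runs a Growth timeline that scales five meshes until a delayed stop triggered from its update.
; After the same delay, AppleLoose destroys those meshes and many Carrot-named components, spawns BP_AppleLoose at a marker point and plays a harvest sound.
; The widget is then hidden; the random grow-time calculation is left unconnected.
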(event Custom|GrowApple
  (bind _plant_size (Timeline|Growth Play)
    (:Update
      (Transformation|SetWorldScale3D (Variables|Default|GetStaticMesh4) (Math|Conversions|ToVector(Float) _plant_size))
      (Utilities|FlowControl|Delay 1e+01)
      (Timeline|Growth Stop))))

(event EventBeginPlay
  (CallFunction|GrowApple)
  (Utilities|FlowControl|Delay 1e+01)
  (CallFunction|AppleLoose)
  (Rendering|SetVisibility (Variables|Default|GetWidget) false false))

(fn ConstructionScript)

(fn AppleLoose
  (Components|DestroyComponent (Variables|Default|GetCarrot52))
  (bind _returnvalue (Game|SpawnActorfromClass "/Game/ActorsBP/CropLoose/ReadyCrops/BP_AppleLoose.BP_AppleLoose_C" (Transformation|GetWorldTransform (Variables|Default|GetAppleLoosePoint)) "Undefined" 0 0))
  (Audio|PlaySound2D "/Game/Sound_Effects/CropingAndHarvestingCropsSounds/HarvestingSound/Harvest_Crop_Activities_2.Harvest_Crop_Activities_2" 1.0 1.0 0.0 0 _returnvalue))