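; Eggplant crop actor that grows on BeginPlay and, after a random delay, turns itself into a loose eggplant actor.
; The Growth timeline scales dozens of individual plant meshes, with a delay in its update path that later stops the timeline.
; When the random delay between the two grow-time variables ends, it destroys the meshes, spawns BP_EggPlantLoose at the EggLoose transform, plays sounds and hides its widget.
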(event Custom|GrowEggPlant
  (bind _plant_size (Timeline|Growth Play)
    (:Update
      (Transformation|SetWorldScale3D (Variables|Default|GetStaticMesh36) (Math|Conversions|ToVector(Float) _plant_size))
      (Utilities|FlowControl|Delay (Variables|Default|GetEggPlantGrowTime))
      (Timeline|Growth Stop))))

(event EventBeginPlay
  (CallFunction|GrowEggPlant)
  (Utilities|FlowControl|Delay (Math|Random|RandomFloatinRange (Variables|Default|GetEggPlantGrowTime) (Variables|Default|GetEggPlantNewGrowTime)))
  (CallFunction|LooseEggPlant)
  (Audio|PlaySound2D "/Game/Sound_Effects/CropingAndHarvestingCropsSounds/Planting_Seeds/Crunch_of_a_Soft_Shell_3.Crunch_of_a_Soft_Shell_3" 1.0 1.0 0.0 0 0)
  (Rendering|SetVisibility (Variables|Default|GetWidget) false false))

(fn ConstructionScript)

(fn LooseEggPlant
  (Components|DestroyComponent (Variables|Default|GetStaticMesh54))
  (bind _returnvalue (Game|SpawnActorfromClass "/Game/ActorsBP/CropLoose/ReadyCrops/BP_EggPlantLoose.BP_EggPlantLoose_C" (Transformation|GetWorldTransform (Variables|Default|GetEggLoose)) "Undefined" 0 0))
  (Audio|PlaySound2D "/Game/Sound_Effects/CropingAndHarvestingCropsSounds/HarvestingSound/Harvest_Crop_Activities_2.Harvest_Crop_Activities_2" 1.0 1.0 0.0 0 _returnvalue))