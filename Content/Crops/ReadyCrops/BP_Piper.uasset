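; Pepper crop actor that grows on spawn, then turns itself into a loose pepper pickup actor.
; GrowPiper runs a timeline that scales dozens of plant meshes by its PlantSize track.
; Five seconds after BeginPlay, LooseCarrot destroys those meshes and spawns PepperLoose at StaticMesh12's transform with box physics disabled, then the widget is hidden.
; The swap runs on a fixed delay, independent of timeline completion.
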(event Custom|GrowPiper
  (bind _plant_size (Timeline|Timeline_0 Play)
    (:Update
      (Transformation|SetWorldScale3D (Variables|Default|GetStaticMesh4) (Math|Conversions|ToVector(Float) _plant_size))
      (Utilities|FlowControl|Delay 5.0)
      (Timeline|Timeline_0 Stop))))

(event EventBeginPlay
  (CallFunction|GrowPiper)
  (Utilities|FlowControl|Delay 5.0)
  (CallFunction|LooseCarrot)
  (Rendering|SetVisibility (Variables|Default|GetWidget) false false))

(fn ConstructionScript)

(fn LooseCarrot
  (Components|DestroyComponent (Variables|Default|GetStaticMesh41))
  (bind _returnvalue (Game|SpawnActorfromClass "/Game/ActorsBP/CropLoose/ReadyCrops/PepperLoose.PepperLoose_C" (Transformation|GetWorldTransform (Variables|Default|GetStaticMesh12)) "Undefined" 0 0))
  (Physics|SetSimulatePhysics (Variables|/Game/ActorsBP/CropLoose/ReadyCrops/PepperLoose.PepperLoose_C|Getbox _returnvalue) false))