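; Orange crop actor that plays a short growth on BeginPlay, then turns into loose oranges.
; GrowCarrot, despite its name, drives the Growth timeline to scale five meshes and stops it via a five-second Delay.
; After a matching delay, OrangeLoose destroys a long hardcoded list of mesh components, spawns BP_OrangesLoose at StaticMesh72's transform, and the widget is hidden.
; The randomized grow time is unused.
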(event Custom|GrowCarrot
  (bind _plant_size (Timeline|Growth Play)
    (:Update
      (Transformation|SetWorldScale3D (Variables|Default|GetStaticMesh) (Math|Conversions|ToVector(Float) _plant_size))
      (Utilities|FlowControl|Delay 5.0)
      (Timeline|Growth Stop))))

(event EventBeginPlay
  (CallFunction|GrowCarrot)
  (Utilities|FlowControl|Delay 5.0)
  (CallFunction|OrangeLoose)
  (Rendering|SetVisibility (Variables|Default|GetWidget) false false))

(fn ConstructionScript)

(fn OrangeLoose
  (Components|DestroyComponent (Variables|Default|GetStaticMesh142))
  (Game|SpawnActorfromClass "/Game/ActorsBP/CropLoose/ReadyCrops/BP_OrangesLoose.BP_OrangesLoose_C" (Transformation|GetWorldTransform (Variables|Default|GetStaticMesh72)) "Undefined" 0 0))