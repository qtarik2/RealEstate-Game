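; BP_WaterMelon is a watermelon crop actor that grows in place, then turns into a loose watermelon.
; On BeginPlay the Growth timeline scales its plant meshes via PlantSize, stopping after WaterMelonGrowTime.
; After a random delay between the two grow-time values, LooseWaterMelon destroys those meshes and spawns BP_WaterMelonLoose at StaticMesh44's transform, then the widget is hidden.
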(event Custom|GrowWaterMelon
  (bind _plant_size (Timeline|Growth Play)
    (:Update
      (Transformation|SetWorldScale3D (Variables|Default|GetSM_Pumpkin_05) (Math|Conversions|ToVector(Float) _plant_size))
      (Utilities|FlowControl|Delay (Variables|Default|GetWaterMelonGrowTime))
      (Timeline|Growth Stop))))

(event EventBeginPlay
  (CallFunction|GrowWaterMelon)
  (Utilities|FlowControl|Delay (Math|Random|RandomFloatinRange (Variables|Default|GetWaterMelonGrowTime) (Variables|Default|GetWaterMelonNewGrowTime)))
  (CallFunction|LooseWaterMelon)
  (Rendering|SetVisibility (Variables|Default|GetWidget) false false))

(fn ConstructionScript)

(fn LooseWaterMelon
  (Components|DestroyComponent (Variables|Default|GetSM_Pumpkin_06))
  (Game|SpawnActorfromClass "/Game/ActorsBP/CropLoose/ReadyCrops/BP_WaterMelonLoose.BP_WaterMelonLoose_C" (Transformation|GetWorldTransform (Variables|Default|GetStaticMesh44)) "Undefined" 0 0))