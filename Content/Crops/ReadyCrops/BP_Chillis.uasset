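; BP_Chillis is a chilli crop that grows, then harvests itself into loose produce.
; On BeginPlay, GrowChillis runs a timeline that scales many plant meshes by PlantSize and is stopped by a delay.
; A fixed delay after BeginPlay, LooseCarrot destroys plant meshes, spawns ChillisLoose at StaticMesh58 and plays a harvest sound, then the widget is hidden.
; The random grow-time calculation is unused.
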(event Custom|GrowChillis
  (bind _plant_size (Timeline|Timeline_0 Play)
    (:Update
      (Transformation|SetWorldScale3D (Variables|Default|GetStaticMesh4) (Math|Conversions|ToVector(Float) _plant_size))
      (Utilities|FlowControl|Delay 5.0)
      (Timeline|Timeline_0 Stop))))

(event EventBeginPlay
  (CallFunction|GrowChillis)
  (Utilities|FlowControl|Delay 5.0)
  (CallFunction|LooseCarrot)
  (Rendering|SetVisibility (Variables|Default|GetWidget) false false))

(fn ConstructionScript)

(fn LooseCarrot
  (Components|DestroyComponent (Variables|Default|GetStaticMesh))
  (Game|SpawnActorfromClass "/Game/ActorsBP/CropLoose/ReadyCrops/ChillisLoose.ChillisLoose_C" (Transformation|GetWorldTransform (Variables|Default|GetStaticMesh58)) "Undefined" 0 0)
  (Audio|PlaySound2D "/Game/Sound_Effects/CropingAndHarvestingCropsSounds/HarvestingSound/Harvest_Crop_Activities_2.Harvest_Crop_Activities_2" 1.0 1.0 0.0 0 0))