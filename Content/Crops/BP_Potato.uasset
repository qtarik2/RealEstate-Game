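; BP_Potato is a potato crop made of about eighty static mesh components that visually grow when play begins.
; BeginPlay calls the GrowPotato event, which plays the Growth timeline.
; Each timeline update converts the PlantSize track into a vector and sets it as the world scale of every mesh at once, so all plants grow in unison.
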(event Custom|GrowPotato
  (bind _plant_size (Timeline|Growth Play)
    (:Update
      (Transformation|SetWorldScale3D (Variables|Default|GetStaticMesh11) (Math|Conversions|ToVector(Float) _plant_size)))))

(event EventBeginPlay
  (CallFunction|GrowPotato))

(fn ConstructionScript)