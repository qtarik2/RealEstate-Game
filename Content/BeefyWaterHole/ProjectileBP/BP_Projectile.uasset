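; Projectile actor for the BeefyWaterHole water system, set up to interact through a BPBeefyInteractionComponent with buoyancy and wake, idle and splash particles.
; The construction script scales the collision mesh, refreshes the component's bounds, then passes it collision, timing, physics and particle settings.
; An optional CelShading flag enables custom depth and stencil on the static mesh.
; BeginPlay and the projectile stop and bounce events are empty.
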(event OnProjectileStop(ProjectileMovement)
  (params (ImpactResult :type Hit%20Result%20Structure%20%28by%20ref%29)))

(event OnProjectileBounce(ProjectileMovement)
  (params (ImpactResult :type Hit%20Result%20Structure%20%28by%20ref%29) (ImpactVelocity :type Vector%20%28by%20ref%29 :default "0, 0, 0")))

(event EventBeginPlay)

(fn ConstructionScript
  (CallFunction|SetProjectileSize (Variables|Default|GetProjectileSize))
  (if (Variables|Default|GetCelShading)
    (Rendering|SetRenderCustomDepth (Variables|Default|GetStaticMesh) true)
    (Rendering|SetCustomDepthStencilValue (Variables|Default|GetStaticMesh) 1)
    (else
      (Rendering|SetRenderCustomDepth (Variables|Default|GetStaticMesh) false)))
  ;[0.2708 0.526 1] Interaction Component Setup
  (Default|InitializeComponent (Variables|Default|GetBP_BeefyInteractionComponent) (Variables|Default|GetStaticMeshCollision) (Variables|Default|GetTimeInterval) (Variables|Default|GetWakeTimeInterval) (Variables|Default|GetIdleTimeInterval) (Variables|Default|GetWakeSpeedLimit) (Variables|Default|GetBuoyantMass) true (Variables|Default|GetEnablePhysics))
  (Default|SetParticles (Variables|Default|GetBP_BeefyInteractionComponent) (Variables|Default|GetWakeParticle) (Variables|Default|GetIdleParticle) (Variables|Default|GetSplashParticle)))

(fn SetProjectileSize
  (params (Size :type Float%20%28single-precision%29))
  (Transformation|SetRelativeScale3D (Variables|Default|GetStaticMeshCollision) (Math|Conversions|ToVector(Float) Size))
  (Default|UpdateComponentBounds (Variables|Default|GetBP_BeefyInteractionComponent)))