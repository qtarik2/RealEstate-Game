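; Master water actor that handles objects entering and leaving water, with splash particles tinted by the material's foam color.
; Overlaps notify the object's BP_BeefyInteractionComponent, or spawn a size-based splash for actors without one.
; Splash height and rotation follow the nearest spline point on spline water, otherwise the water component's transform.
; It also writes landscape bounds to MPC_Level and wakes already-overlapping interaction components shortly after BeginPlay.
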(event EventBeginPlay
  (Setup|GetLandscapeBounds)
  (Setup|SetFoamColor)
  (Utilities|Time|SetTimerbyFunctionName 0 "WakeActorsOnBegin" 0.01))

(event Collision|EventActorBeginOverlap
  (params (OtherActor :type Actor%20Object%20Reference))
  (if (and (Utilities|IsValid OtherActor) (Variables|01.Main|GetObject%20Interactions))
    (Interaction|EnterActor OtherActor)))

(event Collision|EventActorEndOverlap
  (params (OtherActor :type Actor%20Object%20Reference))
  (if (and (Utilities|IsValid OtherActor) (Variables|01.Main|GetObject%20Interactions))
    (Interaction|ExitActor OtherActor)))

(fn ConstructionScript
  (Setup|GetLandscapeBounds)
  (Utilities|IsValid (Variables|01.Main|GetWater%20Material)
    (:Is%20Valid
      (Setup|SetFoamColor))))

(fn GetLandscapeBounds
  (bind _outactors (Actor|GetAllActorsOfClass "/Script/Landscape.Landscape"))
  (if (> (Utilities|Array|Length _outactors) 0)
    (Rendering|Material|SetVectorParameterValue "/Game/BeefyWaterHole/MPC_Level.MPC_Level" "Landscape Max" (Math|Conversions|ToLinearColor(Vector) (Math|Vector|MakeVector (+ (.X (Math|Vector|BreakVector (.Origin (Collision|GetActorBounds (Utilities|Array|Get(acopy) _outactors) false)))) (.X (Math|Vector|BreakVector (.BoxExtent (Collision|GetActorBounds (Utilities|Array|Get(acopy) _outactors) false))))) (+ (.Y (Math|Vector|BreakVector (.Origin (Collision|GetActorBounds (Utilities|Array|Get(acopy) _outactors) false)))) (.Y (Math|Vector|BreakVector (.BoxExtent (Collision|GetActorBounds (Utilities|Array|Get(acopy) _outactors) false))))) (+ (.Z (Math|Vector|BreakVector (.Origin (Collision|GetActorBounds (Utilities|Array|Get(acopy) _outactors) false)))) (.Z (Math|Vector|BreakVector (.BoxExtent (Collision|GetActorBounds (Utilities|Array|Get(acopy) _outactors) false))))))) :!class /Script/Engine.KismetMaterialLibrary)
    (Rendering|Material|SetVectorParameterValue "/Game/BeefyWaterHole/MPC_Level.MPC_Level" "Landscape Min" (Math|Conversions|ToLinearColor(Vector) (Math|Vector|MakeVector (- (.X (Math|Vector|BreakVector (.Origin (Collision|GetActorBounds (Utilities|Array|Get(acopy) _outactors) false)))) (.X (Math|Vector|BreakVector (.BoxExtent (Collision|GetActorBounds (Utilities|Array|Get(acopy) _outactors) false))))) (- (.Y (Math|Vector|BreakVector (.Origin (Collision|GetActorBounds (Utilities|Array|Get(acopy) _outactors) false)))) (.Y (Math|Vector|BreakVector (.BoxExtent (Collision|GetActorBounds (Utilities|Array|Get(acopy) _outactors) false))))) (- (.Z (Math|Vector|BreakVector (.Origin (Collision|GetActorBounds (Utilities|Array|Get(acopy) _outactors) false)))) (.Z (Math|Vector|BreakVector (.BoxExtent (Collision|GetActorBounds (Utilities|Array|Get(acopy) _outactors) false))))))) :!class /Script/Engine.KismetMaterialLibrary)))

(fn SpawnSplashParticle
  (params (ParticleLocation :type Vector) (ParticleSize :type Float%20%28single-precision%29))
  (if (> ParticleSize (Variables|03.Particles|GetParticle%20Size%20Threshold))
    (LocalVariables|SetNewParticle (Variables|03.Particles|GetSplashParticleBig))
    (else
      (LocalVariables|SetNewParticle (Variables|03.Particles|GetSplashParticleSmall))))
  (Particles|SpawnParticleNearLocation (LocalVariables|GetNewParticle) ParticleLocation))

(fn SetFoamColor
  (bind _output_get (Variables|03.Particles|SetFoamColor (Math|Conversions|ToColor(LinearColor) (.parametervalue (Utilities|Array|Get(acopy) (Variables|/Script/Engine.MaterialInstance|GetVectorParameterValues (Variables|01.Main|GetWater%20Material)) (Variables|03.Particles|GetFoamColorIndex))))))
  (return _output_get))

(fn SpawnParticleNearLocation
  (params (NewParticle :type Particle%20System%20Object%20Reference) (ParticleLocation :type Vector))
  (bind (_world_height _particlerotation) (Particles|GetWaterMeshHeight ParticleLocation))
  (LocalVariables|SetParticleHeight _world_height)
  (Particles|SpawnParticle NewParticle (Math|Vector|MakeVector (.x ParticleLocation) (.y ParticleLocation) (LocalVariables|GetParticleHeight)) _particlerotation))

(fn EnterActor
  (params (OtherActor :type Actor%20Object%20Reference))
  (bind _returnvalue (Actor|GetComponentbyClass OtherActor "/Game/BeefyWaterHole/BeefyWater/BlueprintMaster/BP_BeefyInteractionComponent.BP_BeefyInteractionComponent_C"))
  (bind (_origin _boxextent) (Collision|GetActorBounds OtherActor true))
  (if (Utilities|IsValid _returnvalue)
    (Default|EnterWater _returnvalue (Variables|Default|GetWaterComponent) (Variables|03.Particles|GetFoamColor) (Variables|03.Particles|GetWaterSpeed))
    (else
      (Particles|SpawnSplashParticle _origin (.x _boxextent)))))

(fn ExitActor
  (params (OtherActor :type Actor%20Object%20Reference))
  (bind _returnvalue (Actor|GetComponentbyClass OtherActor "/Game/BeefyWaterHole/BeefyWater/BlueprintMaster/BP_BeefyInteractionComponent.BP_BeefyInteractionComponent_C"))
  (bind (_origin _boxextent) (Collision|GetActorBounds OtherActor true))
  (if (Utilities|IsValid _returnvalue)
    (Default|ExitWater _returnvalue)
    (else
      (Particles|SpawnSplashParticle _origin (.x _boxextent)))))

(fn GetWaterMeshHeight
  (params (Location :type Vector))
  (bind _asspline_component (Utilities|Casting|CastToSplineComponent (Variables|Default|GetWaterComponent))
    (:then
      (LocalVariables|SetHeight (.z (Spline|FindLocationClosesttoWorldLocation _asspline_component Location "World")))
      (LocalVariables|SetRotation (Math|Rotator|MakeRotationfromAxes (Spline|FindDirectionClosesttoWorldLocation _asspline_component Location "World") (Math|Vector|CrossProduct (Class|SplineComponent|FindUpVectorClosesttoWorldLocation _asspline_component Location "World") (Spline|FindDirectionClosesttoWorldLocation _asspline_component Location "World")) (Class|SplineComponent|FindUpVectorClosesttoWorldLocation _asspline_component Location "World"))))
    (:CastFailed
      (LocalVariables|SetHeight (.z (Transformation|GetWorldLocation (Variables|Default|GetWaterComponent))))
      (LocalVariables|SetRotation (Transformation|GetWorldRotation (Variables|Default|GetWaterComponent)))))
  (return (LocalVariables|GetHeight) (LocalVariables|GetRotation)))

(fn WakeActorsonBegin
  (for _array_element (Collision|GetOverlappingActors 0 :!class /Script/Engine.Actor)
    (if (> (Utilities|Array|Length (Actor|GetComponentsByClass _array_element "/Game/BeefyWaterHole/BeefyWater/BlueprintMaster/BP_BeefyInteractionComponent.BP_BeefyInteractionComponent_C")) 0)
      (Default|WakeUponBegin (Utilities|Array|Get(acopy) (Actor|GetComponentsByClass _array_element "/Game/BeefyWaterHole/BeefyWater/BlueprintMaster/BP_BeefyInteractionComponent.BP_BeefyInteractionComponent_C")) (Variables|Default|GetWaterComponent) (Variables|03.Particles|GetFoamColor) 3.0 (Variables|03.Particles|GetWaterSpeed)))))

(fn SpawnParticle
  (params (Particle :type Particle%20System%20Object%20Reference) (Location :type Vector) (Rotation :type Rotator))
  (bind _returnvalue (Effects|SpawnEmitteratLocation Particle Location Rotation))
  (Rendering|SetTranslucentSortPriority _returnvalue 10)
  (Effects|Components|ParticleSystem|SetColorParameter _returnvalue "Foam Color" (Math|Conversions|ToLinearColor(Color) (Variables|03.Particles|GetFoamColor)))
  (Effects|Components|ParticleSystem|SetFloatParameter _returnvalue "WaterSpeed" (Variables|03.Particles|GetWaterSpeed)))