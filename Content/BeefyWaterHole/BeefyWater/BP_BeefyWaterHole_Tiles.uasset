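; BP_BeefyWaterHole_Tiles is a water surface actor that builds a TileX by TileY grid of water mesh tiles.
; Its construction script spaces static mesh components by the scaled mesh bounds, centres the grid on the actor origin and scales tiles only in X and Y.
; Each tile gets the water mesh, material and a WorldStatic block response, then joins MeshTiles, with the first stored as WaterComponent.
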(event EventBeginPlay
  (|CallParentFunction) ; This node is disabled and will not be called.\nDrag off pins to build functionality.
)

(event Collision|EventActorBeginOverlap
  (params (OtherActor :type Actor%20Object%20Reference))
  (|CallParentFunction OtherActor) ; This node is disabled and will not be called.\nDrag off pins to build functionality.
)

(event EventTick
  (params (DeltaSeconds :type Float%20%28single-precision%29)))

(fn ConstructionScript
  (bind _tiley (Variables|Default|GetTileY))
  (bind _tilex (Variables|Default|GetTileX))
  (bind _water_mesh (Variables|Default|GetWater%20Mesh))
  (bind _mesh_scale (Variables|Default|GetMesh%20Scale))
  (bind _mesh_scale_2 (Variables|Default|GetMesh%20Scale))
  (bind _returnvalue (- _tiley 1))
  (bind _returnvalue_2 (- _tilex 1))
  (bind _returnvalue_3 (StaticMesh|GetBoundingBox _water_mesh))
  (bind _returnvalue_4 (- (.max _returnvalue_3) (.min _returnvalue_3)))
  (bind _returnvalue_5 (* _returnvalue_4 _mesh_scale))
  (bind _returnvalue_6 (* _returnvalue_2 (.x _returnvalue_5)))
  (bind _returnvalue_7 (* _returnvalue (.y _returnvalue_5)))
  (bind _returnvalue_8 (/ _returnvalue_7 2.0))
  (bind _returnvalue_9 (/ _returnvalue_6 2.0))
  (bind _returnvalue_10 (- "0, 0, 0" (Math|Vector|MakeVector _returnvalue_9 _returnvalue_8 0.0)))
  (|CallParentFunction)
  (Utilities|Array|Clear (Variables|Default|GetMeshTiles))
  (for _index (range 0 (- (Variables|Default|GetTileX) 1))
    (LocalVariables|SetIndexX _index)
    (for _index_2 (range 0 (- (Variables|Default|GetTileY) 1))
      (LocalVariables|SetIndexY _index_2)
      (bind _returnvalue_11 (AddComponent|AddStaticMeshComponent false (Math|Transform|MakeTransform (Math|Vector|MakeVector (+ (.x _returnvalue_10) (* (LocalVariables|GetIndexX) (.x _returnvalue_5))) (+ (.y _returnvalue_10) (* (LocalVariables|GetIndexY) (.y _returnvalue_5))) 0.0) "0, 0, 0" (Math|Vector|MakeVector _mesh_scale_2 _mesh_scale_2 1.0))))
      (Collision|SetCollisionResponsetoChannel _returnvalue_11 "ECC_WorldStatic" "ECR_Block")
      (Rendering|Material|SetMaterial _returnvalue_11 0 (Variables|Default|GetWater%20Material))
      (Components|StaticMesh|SetStaticMesh _returnvalue_11 (Variables|Default|GetWater%20Mesh))
      (Utilities|Array|Add (Variables|Default|GetMeshTiles) _returnvalue_11)))
  (Variables|Default|SetWaterComponent (Utilities|Array|Get(acopy) (Variables|Default|GetMeshTiles))))