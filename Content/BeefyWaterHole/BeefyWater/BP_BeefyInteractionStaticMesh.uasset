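; Static mesh actor for a BeefyWaterHole that produces wake, idle and splash particles through its BP_BeefyInteractionComponent.
; Construction sizes the collision and bounding sphere, configures the component, and toggles custom depth stencil for cel shading.
; With WakeOnCollision, it tracks nearby actors carrying interaction components, starting wading on overlap and stopping when the last leaves.
; At BeginPlay, pawns already nearby wake it with the overlapped water hole's component, foam color and speed.
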(event EventBeginPlay
  ;[1 1 1] Nearby Components
  (bind _asbp_beefy_water_hole (Utilities|Casting|CastToBP_BeefyWaterHole (Utilities|Array|Get(acopy) (Collision|GetOverlappingActors "/Game/BeefyWaterHole/BeefyWater/BlueprintMaster/BP_BeefyWaterHole.BP_BeefyWaterHole_C" :!class /Script/Engine.Actor))))
  (if (Variables|Default|GetWake%20On%20Collision)
    (bind _wake_collision (CallFunction|FindNearbyInteractionComponents))
    (if _wake_collision
      (Default|WakeUp (Variables|Default|GetBP_BeefyInteractionComponent) (Variables|/Game/BeefyWaterHole/BeefyWater/BlueprintMaster/BP_BeefyWaterHole.BP_BeefyWaterHole_C|GetWaterComponent _asbp_beefy_water_hole) (Variables|/Game/BeefyWaterHole/BeefyWater/BlueprintMaster/BP_BeefyWaterHole.BP_BeefyWaterHole_C|GetFoamColor _asbp_beefy_water_hole) 1.0 (Variables|/Game/BeefyWaterHole/BeefyWater/BlueprintMaster/BP_BeefyWaterHole.BP_BeefyWaterHole_C|GetWaterSpeed _asbp_beefy_water_hole)))))

(event Collision|EventActorBeginOverlap
  (params (OtherActor :type Actor%20Object%20Reference))
  ;[1 1 1] Component Collision
  (if (Variables|Default|GetWake%20On%20Collision)
    (bind _nearbyinteraction (CallFunction|IsNewInteractionComponent OtherActor))
    (if _nearbyinteraction
      (Default|StartWadingImmediately (Variables|Default|GetBP_BeefyInteractionComponent)))))

(event EventTick
  (params (DeltaSeconds :type Float%20%28single-precision%29)))

(event Collision|EventActorEndOverlap
  (params (OtherActor :type Actor%20Object%20Reference))
  ;[1 1 1] Component Collision
  (if (Variables|Default|GetWake%20On%20Collision)
    (bind _lastinteraction (CallFunction|IsLastInteractionComponent OtherActor))
    (if _lastinteraction
      (Default|StopWading (Variables|Default|GetBP_BeefyInteractionComponent)))))

(fn ConstructionScript
  (bind _waketimeinterval (Variables|Default|GetWakeTimeInterval))
  (Utilities|Array|Clear (Variables|Default|GetComponentsNearby))
  (Transformation|SetRelativeScale3D (Variables|Default|GetStaticMeshCollision) (Math|Conversions|ToVector(Float) (Variables|Default|GetMeshScale)))
  (Components|Sphere|SetSphereRadius (Variables|Default|GetBoundingSphere) (Variables|Default|GetCollisionRadius) true)
  (if (Variables|Default|GetCelShading)
    (Rendering|SetRenderCustomDepth (Variables|Default|GetStaticMesh) true)
    (Rendering|SetCustomDepthStencilValue (Variables|Default|GetStaticMesh) 1)
    (else
      (Rendering|SetRenderCustomDepth (Variables|Default|GetStaticMesh) false)))
  ;[1 1 1] Interaction Component Setup
  (Default|InitializeComponent (Variables|Default|GetBP_BeefyInteractionComponent) (Variables|Default|GetStaticMeshCollision) 0.1 _waketimeinterval _waketimeinterval 2e+01 1e+02 (not (Variables|Default|GetWake%20On%20Collision)) false)
  (Default|SetParticles (Variables|Default|GetBP_BeefyInteractionComponent) (Variables|Default|GetWakeParticle) (Variables|Default|GetIdleParticle) (Variables|Default|GetSplashParticle)))

(fn IsNewInteractionComponent
  (params (Actor :type Actor%20Object%20Reference))
  (bind _returnvalue (Actor|GetComponentsByClass Actor "/Game/BeefyWaterHole/BeefyWater/BlueprintMaster/BP_BeefyInteractionComponent.BP_BeefyInteractionComponent_C"))
  (bind _output (Utilities|Array|Get(acopy) _returnvalue))
  (if (Utilities|IsValid _output)
    (LocalVariables|SetisInteractionActor true)
    (Utilities|Array|Add (Variables|Default|GetComponentsNearby) _output)
    (else
      (LocalVariables|SetisInteractionActor false)))
  (return (LocalVariables|GetisInteractionActor)))

(fn IsLastInteractionComponent
  (params (Actor :type Actor%20Object%20Reference))
  (bind _returnvalue (Actor|GetComponentsByClass Actor "/Game/BeefyWaterHole/BeefyWater/BlueprintMaster/BP_BeefyInteractionComponent.BP_BeefyInteractionComponent_C"))
  (bind _output (Utilities|Array|Get(acopy) _returnvalue))
  (if (Utilities|IsValid _output)
    (Utilities|Array|RemoveItem (Variables|Default|GetComponentsNearby) _output)
    (if (== (Utilities|Array|Length (Variables|Default|GetComponentsNearby)) 0)
      (LocalVariables|SetisLastInteraction true)
      (else
        (LocalVariables|SetisLastInteraction false :!label _label)))
    (else
      (goto _label)))
  (return (LocalVariables|GetisLastInteraction)))

(fn FindNearbyInteractionComponents
  (for _array_element (Collision|GetOverlappingActors (Variables|Default|GetBoundingSphere) "/Script/Engine.Pawn" :!class /Script/Engine.PrimitiveComponent)
    (if (Utilities|IsValid (Actor|GetComponentbyClass _array_element "/Game/BeefyWaterHole/BeefyWater/BlueprintMaster/BP_BeefyInteractionComponent.BP_BeefyInteractionComponent_C"))
      (Utilities|Array|Add (Variables|Default|GetComponentsNearby) (Actor|GetComponentbyClass _array_element "/Game/BeefyWaterHole/BeefyWater/BlueprintMaster/BP_BeefyInteractionComponent.BP_BeefyInteractionComponent_C"))
      (LocalVariables|SetWakeUpComponent true)))
  (return (LocalVariables|GetWakeUpComponent)))