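; Construction-script tool that fills a rectangular grid, sized by a Corner vector, with rows of grain draped over the surface below.
; AdjustGrid scales the preview grid mesh and clamps the corner.
; CreateGrainRows traces downward at spaced points along each row to build a hidden spline.
; PlantGrain lays spline meshes along it, using dynamic materials with random U offset, length-based U scale and wind, plus optional shadows and cull distance.
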(event EventBeginPlay)

(event Collision|EventActorBeginOverlap
  (params (OtherActor :type Actor%20Object%20Reference)))

(event EventTick
  (params (DeltaSeconds :type Float%20%28single-precision%29)))

(fn ConstructionScript
  (CallFunction|AdjustGrid)
  (if (Variables|Planting|GetPlantCrops)
    (CallFunction|CreateGrainRows)))

(fn AdjustGrid
  ;[1 1 1] Set grid length and width based on corner position
  (Variables|Grid|SetPlanter_Grid_Length (.X (Math|Vector|BreakVector (Variables|Grid|GetCorner))))
  (Variables|Grid|SetPlanter_Grid_Width (.Y (Math|Vector|BreakVector (Variables|Grid|GetCorner))))
  (LocalVariables|SetCornerZ (.Z (Math|Vector|BreakVector (Variables|Grid|GetCorner))))
  ;[1 1 1] Change scale of grid mesh base on position of corner
  (Transformation|SetRelativeScale3D (Variables|Default|GetSM_DmS_Planting_Grid) (Math|Vector|MakeVector (/ (Variables|Grid|GetPlanter_Grid_Width) 1e+02) (/ (Variables|Grid|GetPlanter_Grid_Length) 1e+02) 1.0))
  ;[1 1 1] Set grid visibility
  (Rendering|SetVisibility (Variables|Default|GetSM_DmS_Planting_Grid) (Variables|Grid|GetShowGrid) false)
  ;[1 1 1] If grid length is < 100cm the corner position is reset
  (if (>= (Variables|Grid|GetPlanter_Grid_Length) 1e+02)
    (LocalVariables|SetXReset (Variables|Grid|GetPlanter_Grid_Length))
    (else
      (LocalVariables|SetXReset 1e+02)
      (LocalVariables|SetResetTrigger true)))
  ;[1 1 1] If grid width is < 10cm the corner position is reset
  (if (>= (Variables|Grid|GetPlanter_Grid_Width) 1e+01)
    (LocalVariables|SetYReset (Variables|Grid|GetPlanter_Grid_Width))
    (else
      (LocalVariables|SetYReset 1e+01)
      (LocalVariables|SetResetTrigger true)))
  ;[1 1 1] Reset the Z component of the corner if there is any movement
  (if (== (LocalVariables|GetCornerZ) 0.0)
    _
    (else
      (LocalVariables|SetResetTrigger true)))
  (if (LocalVariables|GetResetTrigger)
    ;[1 1 1] Resets the corner position
    (Variables|Grid|SetCorner (Math|Vector|MakeVector (LocalVariables|GetXReset) (LocalVariables|GetYReset) (LocalVariables|GetZReset)))))

(fn CreateGrainRows
  (bind _planter_grid_length (Variables|Grid|GetPlanter_Grid_Length))
  (bind _sm_dms_planting_grid (Variables|Default|GetSM_DmS_Planting_Grid))
  (bind _pointspacing (Variables|Planting|GetPointSpacing))
  (bind (_remainder _returnvalue) (Math|Float|Division(WholeandRemainder) _planter_grid_length _pointspacing))
  (bind _returnvalue_2 (Transformation|GetWorldRotation _sm_dms_planting_grid))
  (bind (_roll _pitch _yaw) (Math|Rotator|BreakRotator _returnvalue_2))
  ;[1 1 1] Set row coordinate
  (for _index (range 0 (.ReturnValue (Math|Float|Division(WholeandRemainder) (Variables|Grid|GetPlanter_Grid_Width) (Variables|Planting|GetRowSpacing))))
    (LocalVariables|SetRow_coord (* _index (Variables|Planting|GetRowSpacing)))
    ;[1 1 1] Calculate and set point location along row
    (bind _output_get (Variables|Planting|SetLeftOver _remainder))
    (bind _output_get_2 (Variables|Planting|SetSmall_TextureScale (/ _output_get 1e+02)))
    (Variables|Planting|SetSmallSectionUsed (> _output_get_2 0.0))
    (Utilities|Array|Clear (Variables|Planting|GetSplinePoints))
    (for _index_2 (range 0 _returnvalue)
      (LocalVariables|SetGWT (Math|Transform|MakeTransform (Transformation|GetWorldLocation _sm_dms_planting_grid) (Math|Rotator|MakeRotator _roll _pitch (- _yaw 9e+01))))
      ;[1 1 1] Raytrace onto landscape
      (bind (_outhit _returnvalue_3) (Collision|LineTraceByChannel (Math|Transform|TransformLocation (LocalVariables|GetGWT) (Math|Vector|MakeVector (* _index_2 (Variables|Planting|GetPointSpacing)) (LocalVariables|GetRow_coord) 0.0)) (Math|Vector|MakeVector (.X (Math|Vector|BreakVector (Math|Transform|TransformLocation (LocalVariables|GetGWT) (Math|Vector|MakeVector (* _index_2 (Variables|Planting|GetPointSpacing)) (LocalVariables|GetRow_coord) 0.0)))) (.Y (Math|Vector|BreakVector (Math|Transform|TransformLocation (LocalVariables|GetGWT) (Math|Vector|MakeVector (* _index_2 (Variables|Planting|GetPointSpacing)) (LocalVariables|GetRow_coord) 0.0)))) (- (.Z (Math|Vector|BreakVector (Math|Transform|TransformLocation (LocalVariables|GetGWT) (Math|Vector|MakeVector (* _index_2 (Variables|Planting|GetPointSpacing)) (LocalVariables|GetRow_coord) 0.0)))) (Variables|Grid|GetProjectionDistance))) "TraceTypeQuery1" false 0 "None"))
      (if (Variables|Grid|GetShowTrace)
        (Rendering|Debug|DrawDebugLine (.TraceStart (Collision|BreakHitResult _outhit)) (.TraceEnd (Collision|BreakHitResult _outhit)) "(R=0.875000,G=0.089203,B=0.189771,A=1.000000)" 2.0 1e+01))
      (if _returnvalue_3
        ;[1 1 1] Add spline point
        (Utilities|Array|Add (Variables|Planting|GetSplinePoints) (.ImpactPoint (Collision|BreakHitResult _outhit)))))
    ;[1 1 1] Creat last spline point in row
    (bind (_outhit_2 _returnvalue_4) (Collision|LineTraceByChannel (Math|Transform|TransformLocation (LocalVariables|GetGWT) (Math|Vector|MakeVector (Variables|Grid|GetPlanter_Grid_Length) (LocalVariables|GetRow_coord) 0.0)) (Math|Vector|MakeVector (.X (Math|Vector|BreakVector (Math|Transform|TransformLocation (LocalVariables|GetGWT) (Math|Vector|MakeVector (Variables|Grid|GetPlanter_Grid_Length) (LocalVariables|GetRow_coord) 0.0)))) (.Y (Math|Vector|BreakVector (Math|Transform|TransformLocation (LocalVariables|GetGWT) (Math|Vector|MakeVector (Variables|Grid|GetPlanter_Grid_Length) (LocalVariables|GetRow_coord) 0.0)))) (- (.Z (Math|Vector|BreakVector (Math|Transform|TransformLocation (LocalVariables|GetGWT) (Math|Vector|MakeVector (Variables|Grid|GetPlanter_Grid_Length) (LocalVariables|GetRow_coord) 0.0)))) (Variables|Grid|GetProjectionDistance))) "TraceTypeQuery1" false 0 "None"))
    (if (Variables|Grid|GetShowTrace)
      (Rendering|Debug|DrawDebugLine (.TraceStart (Collision|BreakHitResult _outhit_2)) (.TraceEnd (Collision|BreakHitResult _outhit_2)) "(R=0.875000,G=0.089203,B=0.189771,A=1.000000)" 2.0 1e+01))
    (if _returnvalue_4
      ;[1 1 1] Add last spline point
      (Utilities|Array|Add (Variables|Planting|GetSplinePoints) (.ImpactPoint (Collision|BreakHitResult _outhit_2)))
      ;[1 1 1] Create spline
      (bind _returnvalue_5 (AddComponent|AddSplineComponent false))
      (bind _output_get_3 (LocalVariables|SetNewLocalVar_0 _returnvalue_5))
      (Spline|SetSplinePoints _output_get_3 (Variables|Planting|GetSplinePoints) "World" true)
      ;[1 1 1] Call Plant Grain Function
      (CallFunction|PlantGrain (LocalVariables|GetNewLocalVar_0))
      ;[1 1 1] Set visibility
      (Rendering|SetVisibility (LocalVariables|GetNewLocalVar_0) false false))))

(fn PlantGrain
  (params (RowSpline :type Spline%20Component%20Object%20Reference))
  ;[1 1 1] Set index range for splinemesh creation loop
  (bind _output_get (LocalVariables|SetTempSpline RowSpline))
  (bind _output_get_2 (LocalVariables|SetNumPointsMinus2 (- (Spline|GetNumberOfSplinePoints _output_get) 2)))
  ;[1 1 1] Splinemesh creation loop
  (for _index (range 0 _output_get_2)
    (LocalVariables|SetLoopIndex1 _index)
    (if (not (and (< (Variables|Planting|GetSmall_TextureScale) 1.0) (== (LocalVariables|GetNumPointsMinus2) (LocalVariables|GetLoopIndex1))))
      (Utilities|FlowControl|Sequence
        (:then_0
          ;[1 1 1] Set tiling offset  so grain row maps do not line up to create lines
          (LocalVariables|SetRandomUoffset (Math|Random|RandomFloat))
          ;[1 1 1] Create large section Vine material Instance
          (if (>= (Variables|Grid|GetPlanter_Grid_Length) (Variables|Planting|GetPointSpacing))
            (bind _returnvalue (Rendering|Material|CreateDynamicMaterialInstance (Variables|Planting|GetGrainMaterial) "None" :!class /Script/Engine.KismetMaterialLibrary))
            (bind _output_get_3 (LocalVariables|SetLgSectMat _returnvalue))
            (Rendering|Material|SetScalarParameterValue _output_get_3 "Uoffset" (LocalVariables|GetRandomUoffset) :!class /Script/Engine.MaterialInstanceDynamic)
            (Rendering|Material|SetScalarParameterValue (LocalVariables|GetLgSectMat) "WindVar" (Variables|Planting|GetWind_Strength) :!class /Script/Engine.MaterialInstanceDynamic)
            (Rendering|Material|SetScalarParameterValue (LocalVariables|GetLgSectMat) "Uscale" (/ (Variables|Planting|GetPointSpacing) 1e+02) :!class /Script/Engine.MaterialInstanceDynamic))
          ;[1 1 1] Create small section material instance
          (if (Variables|Planting|GetSmallSectionUsed)
            (bind _returnvalue_2 (Rendering|Material|CreateDynamicMaterialInstance (Variables|Planting|GetGrainMaterial) "None" :!class /Script/Engine.KismetMaterialLibrary))
            (bind _output_get_4 (LocalVariables|SetSmallSectMat _returnvalue_2))
            (Rendering|Material|SetScalarParameterValue _output_get_4 "Uoffset" (LocalVariables|GetRandomUoffset) :!class /Script/Engine.MaterialInstanceDynamic)
            (Rendering|Material|SetScalarParameterValue (LocalVariables|GetSmallSectMat) "WindVar" (Variables|Planting|GetWind_Strength) :!class /Script/Engine.MaterialInstanceDynamic)
            (Rendering|Material|SetScalarParameterValue (LocalVariables|GetSmallSectMat) "Uscale" (Variables|Planting|GetSmall_TextureScale) :!class /Script/Engine.MaterialInstanceDynamic)))
        (:then_1
          ;[1 1 1] Add splinemesh component
          (bind _returnvalue_3 (AddComponent|AddSplineMeshComponent false))
          (bind _output_get_5 (LocalVariables|SetNewLocalVar_1 _returnvalue_3))
          (Transformation|AttachComponentToComponent _output_get_5 (Variables|Default|GetRoot) "None" "KeepWorld" "KeepWorld" "KeepWorld" true)
          ;[1 1 1] Check if last spline point and small section
          (if (and (== (LocalVariables|GetLoopIndex1) (LocalVariables|GetNumPointsMinus2)) (Variables|Planting|GetSmallSectionUsed))
            ;[1 1 1] Set material based on previous branch
            (Rendering|Material|SetMaterial (LocalVariables|GetNewLocalVar_1) 0 (LocalVariables|GetSmallSectMat))
            (else
              (Rendering|Material|SetMaterial (LocalVariables|GetNewLocalVar_1) 0 (LocalVariables|GetLgSectMat))))
          ;[1 1 1] Set start and end points for splinemesh
          (SplineMesh|SetStartandEnd (LocalVariables|GetNewLocalVar_1) (.Location (Spline|GetLocationandTangentatSplinePoint (LocalVariables|GetTempSpline) (LocalVariables|GetLoopIndex1) "Local")) (.Tangent (Spline|GetLocationandTangentatSplinePoint (LocalVariables|GetTempSpline) (LocalVariables|GetLoopIndex1) "Local")) (.Location (Spline|GetLocationandTangentatSplinePoint (LocalVariables|GetTempSpline) (+ (LocalVariables|GetLoopIndex1) 1) "Local")) (.Tangent (Spline|GetLocationandTangentatSplinePoint (LocalVariables|GetTempSpline) (+ (LocalVariables|GetLoopIndex1) 1) "Local")) true :!class /Script/Engine.SplineMeshComponent)
          ;[1 1 1] Set visibility
          (Rendering|SetVisibility (LocalVariables|GetTempSpline) false false)
          ;[1 1 1] Set cast shadow based on user input
          (Rendering|SetCastShadow (LocalVariables|GetNewLocalVar_1) (Variables|Planting|GetCast%20Shadow))
          ;[1 1 1] Set draw distance
          (if (Variables|DrawDistance|GetEnable_Draw_Distance)
            (Class|PrimitiveComponent|SetCullDistance (LocalVariables|GetNewLocalVar_1) (Variables|DrawDistance|GetMax_Draw_Distance))))))))