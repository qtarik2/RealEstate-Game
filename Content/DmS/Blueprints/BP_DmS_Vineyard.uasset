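; Vineyard row actor that procedurally builds a terrain-following grapevine trellis from its origin to EndPoint in the construction script.
; TrellisPath traces downward every 6 m, plus a shorter 2 m-multiple remainder, to build a spline and tiling-scaled material instances.
; Posts places end and randomly yawed middle posts at spline points, and AddVines bridges them with colliding spline meshes.
; GrapeType selects red, green, bare or custom material; draw-distance culling is optional.
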(event EventBeginPlay)

(event Collision|EventActorBeginOverlap
  (params (OtherActor :type Actor%20Object%20Reference)))

(event EventTick
  (params (DeltaSeconds :type Float%20%28single-precision%29)))

(fn ConstructionScript
  (CallFunction|PickGrapeType)
  (CallFunction|TrellisPath)
  (CallFunction|Posts)
  (CallFunction|AddVines))

(fn TrellisPath
  (bind _returnvalue (Transformation|GetActorLocation))
  (bind _guide (Variables|Default|GetGuide))
  (bind _returnvalue_2 (Transformation|GetWorldRotation _guide))
  (bind (_roll _pitch _yaw) (Math|Rotator|BreakRotator _returnvalue_2))
  ;[1 1 1] Clear spline points
  (Utilities|Array|Clear (Variables|Default|GetSplinePoints))
  (Utilities|FlowControl|Sequence
    (:then_0
      ;[1 1 1] Get Grid's world transform using only the x and y components
      (LocalVariables|SetGuide_world_Transform (Math|Transform|MakeTransform (Transformation|GetWorldLocation _guide) (Math|Rotator|MakeRotator _roll _pitch (- _yaw 0.0)))))
    (:then_1
      ;[1 1 1] Set Vine's relative rotation by getting the rotation from the root to the endpoint using only the Z component
      (Variables|Default|SetVineRotation (Math|Rotator|MakeRotator 0.0 0.0 (.Yaw (Math|Rotator|BreakRotator (Math|Rotator|FindLookatRotation _returnvalue (+ _returnvalue (Variables|Guide|GetEndPoint)))))))
      (Transformation|SetRelativeRotation (Variables|Default|GetGuide) (Variables|Default|GetVineRotation) false false))
    (:then_2
      ;[1 1 1] Get the X and Y Vectors of the End Point
      (LocalVariables|SetEndP_X (.X (Math|Vector|BreakVector (Variables|Guide|GetEndPoint))))
      (LocalVariables|SetEndP_Y (.Y (Math|Vector|BreakVector (Variables|Guide|GetEndPoint))))
      ;[1 1 1] Comment
      (Variables|Default|SetVineyardLength (Math|Vector|VectorLength (Math|Vector|MakeVector (LocalVariables|GetEndP_X) (LocalVariables|GetEndP_Y) 0.0)))
      (Transformation|SetRelativeScale3D (Variables|Default|GetGuide) (Math|Vector|MakeVector (/ (Variables|Default|GetVineyardLength) 2e+02) 1.0 1.0)))
    (:then_3
      ;[1 1 1] Keep the relative Z height of the end point at zero
      (Variables|Guide|SetEndPoint (Math|Vector|MakeVector (LocalVariables|GetEndP_X) (LocalVariables|GetEndP_Y) 0.0))
      ;[1 1 1] set num of 6m sectionss
      (bind _output_get (LocalVariables|SetNumLgSecs (.ReturnValue (Math|Float|Division(WholeandRemainder) (Variables|Default|GetVineyardLength) 6e+02))))
      ;[1 1 1] Calculate points tuse use for line trace
      (for _index (range 0 _output_get)
        ;[1 1 1] Line trace to find spline point on terrain
        (bind _outhit (Collision|LineTraceByChannel (Math|Transform|TransformLocation (LocalVariables|GetGuide_world_Transform) (Math|Vector|MakeVector (* (.X (Math|Vector|BreakVector (Variables|Guide|GetEndPoint))) (/ (* _index 6e+02) (Variables|Default|GetVineyardLength))) (* (.Y (Math|Vector|BreakVector (Variables|Guide|GetEndPoint))) (/ (* _index 6e+02) (Variables|Default|GetVineyardLength))) 0.0)) (Math|Vector|MakeVector (.X (Math|Vector|BreakVector (Math|Transform|TransformLocation (LocalVariables|GetGuide_world_Transform) (Math|Vector|MakeVector (* (.X (Math|Vector|BreakVector (Variables|Guide|GetEndPoint))) (/ (* _index 6e+02) (Variables|Default|GetVineyardLength))) (* (.Y (Math|Vector|BreakVector (Variables|Guide|GetEndPoint))) (/ (* _index 6e+02) (Variables|Default|GetVineyardLength))) 0.0)))) (.Y (Math|Vector|BreakVector (Math|Transform|TransformLocation (LocalVariables|GetGuide_world_Transform) (Math|Vector|MakeVector (* (.X (Math|Vector|BreakVector (Variables|Guide|GetEndPoint))) (/ (* _index 6e+02) (Variables|Default|GetVineyardLength))) (* (.Y (Math|Vector|BreakVector (Variables|Guide|GetEndPoint))) (/ (* _index 6e+02) (Variables|Default|GetVineyardLength))) 0.0)))) (- (.Z (Math|Vector|BreakVector (Math|Transform|TransformLocation (LocalVariables|GetGuide_world_Transform) (Math|Vector|MakeVector (* (.X (Math|Vector|BreakVector (Variables|Guide|GetEndPoint))) (/ (* _index 6e+02) (Variables|Default|GetVineyardLength))) (* (.Y (Math|Vector|BreakVector (Variables|Guide|GetEndPoint))) (/ (* _index 6e+02) (Variables|Default|GetVineyardLength))) 0.0)))) 1e+04)) "TraceTypeQuery1" false 0 "None"))
        ;[1 1 1] Add spline point base on line trace hit location
        (Utilities|Array|Add (Variables|Default|GetSplinePoints) (Math|Vector|MakeVector (.X (Math|Vector|BreakVector (.ImpactPoint (Collision|BreakHitResult _outhit)))) (.Y (Math|Vector|BreakVector (.ImpactPoint (Collision|BreakHitResult _outhit)))) (- (.Z (Math|Vector|BreakVector (.ImpactPoint (Collision|BreakHitResult _outhit)))) 1e+01))))
      ;[1 1 1] Calculate length of 2m sections
      (LocalVariables|SetLength_2m (* (.ReturnValue (Math|Float|Division(WholeandRemainder) (Variables|Default|GetVineyardLength) 2e+02)) 2e+02))
      (LocalVariables|SetLength_6m (* (LocalVariables|GetNumLgSecs) 6e+02))
      ;[1 1 1] Compare 2m vs 6m lengths
      (if (> (LocalVariables|GetLength_2m) (LocalVariables|GetLength_6m))
        ;[1 1 1] Set small section texture scale
        (LocalVariables|SetSmallSectionScale (/ (- (LocalVariables|GetLength_2m) (LocalVariables|GetLength_6m)) 2e+02))
        ;[1 1 1] Create final spline point if not a multiple of 6m but a multiple of 2m
        (LocalVariables|Set2m_Div_VineLen (/ (LocalVariables|GetLength_2m) (Variables|Default|GetVineyardLength)))
        (Variables|Default|SetSmallSectionUsed true)
        (bind _outhit_2 (Collision|LineTraceByChannel (Math|Transform|TransformLocation (LocalVariables|GetGuide_world_Transform) (Math|Vector|MakeVector (* (.X (Math|Vector|BreakVector (Variables|Guide|GetEndPoint))) (LocalVariables|Get2m_Div_VineLen)) (* (.Y (Math|Vector|BreakVector (Variables|Guide|GetEndPoint))) (LocalVariables|Get2m_Div_VineLen)) 0.0)) (Math|Vector|MakeVector (.X (Math|Vector|BreakVector (Math|Transform|TransformLocation (LocalVariables|GetGuide_world_Transform) (Math|Vector|MakeVector (* (.X (Math|Vector|BreakVector (Variables|Guide|GetEndPoint))) (LocalVariables|Get2m_Div_VineLen)) (* (.Y (Math|Vector|BreakVector (Variables|Guide|GetEndPoint))) (LocalVariables|Get2m_Div_VineLen)) 0.0)))) (.Y (Math|Vector|BreakVector (Math|Transform|TransformLocation (LocalVariables|GetGuide_world_Transform) (Math|Vector|MakeVector (* (.X (Math|Vector|BreakVector (Variables|Guide|GetEndPoint))) (LocalVariables|Get2m_Div_VineLen)) (* (.Y (Math|Vector|BreakVector (Variables|Guide|GetEndPoint))) (LocalVariables|Get2m_Div_VineLen)) 0.0)))) (- (.Z (Math|Vector|BreakVector (Math|Transform|TransformLocation (LocalVariables|GetGuide_world_Transform) (Math|Vector|MakeVector (* (.X (Math|Vector|BreakVector (Variables|Guide|GetEndPoint))) (LocalVariables|Get2m_Div_VineLen)) (* (.Y (Math|Vector|BreakVector (Variables|Guide|GetEndPoint))) (LocalVariables|Get2m_Div_VineLen)) 0.0)))) 1e+04)) "TraceTypeQuery1" false 0 "None"))
        ;[1 1 1] Add final spline point at line trace hit location
        (Utilities|Array|Add (Variables|Default|GetSplinePoints) (Math|Vector|MakeVector (.X (Math|Vector|BreakVector (.ImpactPoint (Collision|BreakHitResult _outhit_2)))) (.Y (Math|Vector|BreakVector (.ImpactPoint (Collision|BreakHitResult _outhit_2)))) (- (.Z (Math|Vector|BreakVector (.ImpactPoint (Collision|BreakHitResult _outhit_2)))) 1e+01)))
        (else
          (Variables|Default|SetSmallSectionUsed false)))
      ;[1 1 1] Create spline for vineyard using spline point array created from line traces
      (bind _returnvalue_3 (AddComponent|AddSplineComponent false))
      (Spline|ClearSplinePoints _returnvalue_3 true)
      (Spline|SetSplinePoints _returnvalue_3 (Variables|Default|GetSplinePoints) "World" true)
      (Variables|Default|SetVineSpline _returnvalue_3)
      ;[1 1 1] If the vine length is greater than 600 cm create the large section Vine material instance
      (if (>= (Variables|Default|GetVineyardLength) 6e+02)
        (bind _returnvalue_4 (Rendering|Material|CreateDynamicMaterialInstance (Variables|VineMaterial|GetGrapevineMaterial) "None" :!class /Script/Engine.KismetMaterialLibrary))
        (Variables|Default|SetLargeSectionInstance _returnvalue_4)
        ;[1 1 1] Tile material times 3
        (Rendering|Material|SetScalarParameterValue _returnvalue_4 "Uscale" 3.0 :!class /Script/Engine.MaterialInstanceDynamic))
      ;[1 1 1] If there is a vine section at least 200 cm and less than 600 cm create the small section material instance and set the appropriate tiling
      (if (Variables|Default|GetSmallSectionUsed)
        (bind _returnvalue_5 (Rendering|Material|CreateDynamicMaterialInstance (Variables|VineMaterial|GetGrapevineMaterial) "None" :!class /Script/Engine.KismetMaterialLibrary))
        (Variables|Default|SetSmallSectionInstance _returnvalue_5)
        (Rendering|Material|SetScalarParameterValue _returnvalue_5 "Uscale" (LocalVariables|GetSmallSectionScale) :!class /Script/Engine.MaterialInstanceDynamic)))))

(fn AddVines
  ;[1 1 1] Calculate last index for loop through spline points
  (bind _output_get (LocalVariables|SetSpline_Num_2 (- (Spline|GetNumberOfSplinePoints (Variables|Default|GetVineSpline)) 2)))
  ;[1 1 1] Loop for adding splinemeshes
  (for _index (range 0 _output_get)
    (LocalVariables|SetSplinePointIndex _index)
    ;[1 1 1] Add spline mesh component and set collison
    (bind _returnvalue (AddComponent|AddSplineMeshComponent false))
    (bind _output_get_2 (LocalVariables|SetNewLocalVar_2 _returnvalue))
    (Collision|SetCollisionEnabled _output_get_2 "QueryAndPhysics")
    (Collision|SetCollisionResponsetoAllChannels (LocalVariables|GetNewLocalVar_2) "ECR_Block")
    (Transformation|AttachComponentToComponent (LocalVariables|GetNewLocalVar_2) (Variables|Default|GetRoot) "None" "KeepWorld" "KeepWorld" "KeepWorld" true)
    ;[1 1 1] Check if it is last point and in a small section
    (if (and (== (LocalVariables|GetSplinePointIndex) (LocalVariables|GetSpline_Num_2)) (Variables|Default|GetSmallSectionUsed))
      ;[1 1 1] Set material instance to small section
      (Rendering|Material|SetMaterial (LocalVariables|GetNewLocalVar_2) 0 (Variables|Default|GetSmallSectionInstance))
      (else
        ;[1 1 1] set material instance for large vine sections
        (Rendering|Material|SetMaterial (LocalVariables|GetNewLocalVar_2) 0 (Variables|Default|GetLargeSectionInstance))))
    ;[1 1 1] Set the starting and ending points of the splinemesh
    (SplineMesh|SetStartandEnd (LocalVariables|GetNewLocalVar_2) (Spline|GetLocationatSplinePoint (Variables|Default|GetVineSpline) (LocalVariables|GetSplinePointIndex) "Local") "0.000000,1.000000,0.000000" (Spline|GetLocationatSplinePoint (Variables|Default|GetVineSpline) (+ (LocalVariables|GetSplinePointIndex) 1) "Local") "0.000000,1.000000,0.000000" true :!class /Script/Engine.SplineMeshComponent)
    (if (Variables|DrawDistance|GetEnable_Draw_Distance)
      (Class|PrimitiveComponent|SetCullDistance (LocalVariables|GetNewLocalVar_2) (Variables|DrawDistance|GetMax_Draw_Distance)))))

(fn Posts
  (bind _vinespline (Variables|Default|GetVineSpline))
  (bind _returnvalue (Spline|GetNumberOfSplinePoints _vinespline))
  (bind _returnvalue_2 (- _returnvalue 1))
  ;[1 1 1] Comment
  (LocalVariables|SetSpline_Point_Index _returnvalue_2)
  (for _index (range 0 _returnvalue_2)
    (bind _output_get (LocalVariables|SetPost_Index _index))
    ;[1 1 1] check if post index = 0
    (if (== _output_get 0)
      ;[1 1 1] Create starting post
      (bind _returnvalue_3 (AddComponent|AddStaticMeshComponent false (Math|Transform|MakeTransform (Spline|GetLocationatSplinePoint (Variables|Default|GetVineSpline) (LocalVariables|GetPost_Index) "Local") (Variables|Default|GetVineRotation))))
      (Transformation|AttachComponentToComponent _returnvalue_3 (Variables|Default|GetGuide) "None" "KeepWorld" "KeepWorld" "KeepWorld" true)
      (Components|StaticMesh|SetStaticMesh _returnvalue_3 "/Game/DmS/Meshes/SM_DmS_EndPost.SM_DmS_EndPost")
      ;[1 1 1] Set draw distance for starting post
      (if (Variables|DrawDistance|GetEnable_Draw_Distance)
        (Class|PrimitiveComponent|SetCullDistance _returnvalue_3 (Variables|DrawDistance|GetMax_Draw_Distance)))
      (else
        ;[1 1 1] Check if post and spline point index equal each other
        (if (== (LocalVariables|GetPost_Index) (LocalVariables|GetSpline_Point_Index))
          ;[1 1 1] Add end post
          (bind _returnvalue_4 (AddComponent|AddStaticMeshComponent false (Math|Transform|MakeTransform (Spline|GetLocationatSplinePoint (Variables|Default|GetVineSpline) (LocalVariables|GetPost_Index) "Local") (Math|Rotator|MakeRotator 0.0 0.0 (+ (.Yaw (Math|Rotator|BreakRotator (Variables|Default|GetVineRotation))) 1.8e+02)))))
          (Transformation|AttachComponentToComponent _returnvalue_4 (Variables|Default|GetGuide) "None" "KeepWorld" "KeepWorld" "KeepWorld" true)
          (Components|StaticMesh|SetStaticMesh _returnvalue_4 "/Game/DmS/Meshes/SM_DmS_EndPost.SM_DmS_EndPost")
          ;[1 1 1] Set draw distance for end post
          (if (Variables|DrawDistance|GetEnable_Draw_Distance)
            (Class|PrimitiveComponent|SetCullDistance _returnvalue_4 (Variables|DrawDistance|GetMax_Draw_Distance)))
          (else
            ;[1 1 1] Add middle post mesh
            (bind _returnvalue_5 (AddComponent|AddStaticMeshComponent false (Math|Transform|MakeTransform (Spline|GetLocationatSplinePoint (Variables|Default|GetVineSpline) (LocalVariables|GetPost_Index) "Local") (Math|Rotator|MakeRotator 0.0 0.0 (Math|Random|RandomFloatinRange 0.0 359.0)))))
            (Transformation|AttachComponentToComponent _returnvalue_5 (Variables|Default|GetGuide) "None" "KeepWorld" "KeepWorld" "KeepWorld" true)
            (Components|StaticMesh|SetStaticMesh _returnvalue_5 "/Game/DmS/Meshes/SM_DmS_Post.SM_DmS_Post")
            ;[1 1 1] Set draw distance for middle post
            (if (Variables|DrawDistance|GetEnable_Draw_Distance)
              (Class|PrimitiveComponent|SetCullDistance _returnvalue_5 (Variables|DrawDistance|GetMax_Draw_Distance)))))))))

(fn PickGrapeType
  ;[1 1 1] Set  Red grape material
  (if (Utilities|Enum|Equal(Enum) (Variables|VineMaterial|GetGrapeType) "NewEnumerator0")
    (Variables|VineMaterial|SetGrapevineMaterial (Variables|VineMaterial|GetRedGrapeMaterial))
    (else
      ;[1 1 1] Set Green Grape Material
      (if (Utilities|Enum|Equal(Enum) (Variables|VineMaterial|GetGrapeType) "NewEnumerator1")
        (Variables|VineMaterial|SetGrapevineMaterial (Variables|VineMaterial|GetGreenGrapeMaterial))
        (else
          ;[1 1 1] Set bare branch material
          (if (Utilities|Enum|Equal(Enum) (Variables|VineMaterial|GetGrapeType) "NewEnumerator2")
            (Variables|VineMaterial|SetGrapevineMaterial (Variables|VineMaterial|GetBareVineMaterial))
            (else
              ;[1 1 1] Set Custom Material
              (if (Utilities|Enum|Equal(Enum) (Variables|VineMaterial|GetGrapeType) "NewEnumerator3")
                (Variables|VineMaterial|SetGrapevineMaterial (Variables|VineMaterial|GetCustom_Material))))))))))